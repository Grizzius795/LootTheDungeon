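; BP_Item is a world item actor that can be picked up and attached to another component.
; Its construction script looks up item data by name to set the static mesh, clearing it when the data is invalid.
; Interaction through BPC_Interactible sends a PickUpItem interface message to the perpetrator.
; Attach and detach functions toggle physics and collision, snapping location and rotation on attach and keeping world transform on release.
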(event `self.ReceiveBeginPlay`)

(event `self.BPC_Interactible.OnInteract`
  (params (Perpetrator :type "Actor Object Reference"))
  (message `/Game/Items/BPI_Items.Pick Up Item` Perpetrator self))

(fn `AttachToComponent`
  (params (Parent :type "SceneComponent Object Reference"))
  (`PrimitiveComponent.SetSimulatePhysics` (`self.StaticMesh`) false)
  (`self.SetActorEnableCollision` false)
  (`self.K2_AttachToComponent` Parent "None" "SnapToTarget" "SnapToTarget" "KeepRelative"))

(fn `DetachFromParent`
  (`self.K2_DetachFromActor` "KeepWorld" "KeepWorld" "KeepWorld")
  (`PrimitiveComponent.SetSimulatePhysics` (`self.StaticMesh`) true)
  (`self.SetActorEnableCollision` true))

(fn `SetItem`
  (params (ItemName :type Name))
  (bind (_out_data _is_valid) (`/Game/Items/BPFL_Items.GetItemData` ItemName))
  (bind _staticmesh (`self.StaticMesh`))
  (if _is_valid
    (`StaticMeshComponent.SetStaticMesh` _staticmesh (`.Mesh_8_30BF231249DF68B153E86D982AE2D2B3` (break `/Game/Items/Struct_Item` _out_data)))
    (else
      (`StaticMeshComponent.SetStaticMesh` _staticmesh null))))

(fn `UserConstructionScript`
  (`self.SetItem` (`self.Item`)))