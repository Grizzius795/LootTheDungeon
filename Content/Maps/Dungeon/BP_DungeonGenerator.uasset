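; Procedural dungeon generator that builds a room graph from a first room to an end room.
; It adds random compatible content rooms until a minimum count, then places the end room at a corridor door.
; A valid layout needs a long enough start-to-end path; doors or walls come from a data table by type.
; Post-generation sets up the quest, spawns weighted-random mobs and portal traps at tagged points, then spawns players.
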(event `self.ReceiveBeginPlay`)

(event `self.OnPostGeneration`
  (`self.SetupQuest`)
  (`self.SpawnCreatures`)
  (`self.SpawnTraps`)
  (bind _returnvalue (`GameplayStatics.GetActorOfClass` "/Game/Maps/Dungeon/Rooms/BP_DungeonStart.BP_DungeonStart_C"))
  (`/Engine/EditorBlueprintResources/StandardMacros.IsValid` _returnvalue
    (:`Is Valid`
      (`/Game/Maps/Dungeon/Rooms/BP_DungeonStart.SpawnPlayers` _returnvalue)
      (`self.FinishedGeneration`))))

(fn `ChooseDoor`
  (params (CurrentRoom :type "RoomData Object Reference") (CurrentRoomInstance :type "Room Object Reference") (NextRoom :type "RoomData Object Reference") (NextRoomInstance :type "Room Object Reference") (DoorType :type "DoorType Object Reference") (OtherDoorType :type "DoorType Object Reference"))
  (returns (Flipped :type Boolean) (ReturnValue :type "Actor Class Reference"))
  (locals (DoorData :type "/Game/Maps/Dungeon/Rooms/Struct_Door Structure"))
  (set `local.DoorData` (`self.GetDoorTypeData` (`local.DoorType`)))
  (if (and (`KismetSystemLibrary.IsValid` CurrentRoom) (`KismetSystemLibrary.IsValid` NextRoom))
    (return false (`KismetArrayLibrary.Array_Random` (`.Doors_8_487989674DE0DBB2A211B8837BD728C7` (break `/Game/Maps/Dungeon/Rooms/Struct_Door` (`local.DoorData`)))))
    (else
      (return false (`KismetArrayLibrary.Array_Random` (`.Walls_9_B5CB6FB849BDE56D6D9250A2AC60A0A3` (break `/Game/Maps/Dungeon/Rooms/Struct_Door` (`local.DoorData`))))))))

(fn `ChooseFirstRoomData`
  (returns (Transform :type "RoomTransform Structure") (ReturnValue :type "RoomData Object Reference"))
  (return (struct) (`self.FirstRoom`)))

(fn `ChooseNextRoomData`
  (params (CurrentRoom :type "RoomData Object Reference") (CurrentRoomInstance :type "ReadOnlyRoom Interface (by ref)") (DoorData :type "DoorDef Structure (by ref)"))
  (returns (DoorIndex :type Integer) (ReturnValue :type "RoomData Object Reference"))
  (locals (NewRoom :type "RoomData Object Reference"))
  (if (>= (`DungeonGraph.Count` (`self.Graph`)) (`self.MinNbRooms`))
    (if (== (`.Type` (break `DoorDef` (`local.DoorData`))) "/Game/Maps/Dungeon/Rooms/LushLabyrinth/Doors/Door_Corridor.Door_Corridor")
      (return 0 (`self.EndRoom`))
      (else
        _)))
  (bind _returnvalue (`self.GetRandomRoomData` (`self.ContentRooms`) :!label _label))
  (set `local.NewRoom` _returnvalue)
  (if (> (`KismetArrayLibrary.Array_Length` (`RoomData.GetCompatibleDoors` (`local.NewRoom`) (`local.DoorData`))) 0)
    (return -1 (`local.NewRoom`))
    (else
      (goto _label))))

(fn `ContinueToAddRoom`
  (returns (ReturnValue :type Boolean))
  (return (not (`DungeonGraph.HasAlreadyRoomData` (`self.Graph`) (`self.EndRoom`)))))

(fn `GetDoorTypeData`
  (params (DoorType :type "Object Object Reference"))
  (returns (Data :type "/Game/Maps/Dungeon/Rooms/Struct_Door Structure"))
  (bind _outrownames (`DataTableFunctionLibrary.GetDataTableRowNames` "/Game/Maps/Dungeon/Rooms/DT_Doors.DT_Doors"))
  (for _array_element _outrownames
    (bind _returnvalue (`|GetDataTableRow` "/Game/Maps/Dungeon/Rooms/DT_Doors.DT_Doors" _array_element)
      (:`then`
        (if (== (`.DoorType_2_E555F705418FC125B1220792C40D32CB` (break `/Game/Maps/Dungeon/Rooms/Struct_Door` _returnvalue)) DoorType)
          (return _returnvalue))))))

(fn `IsValidDungeon`
  (returns (ReturnValue :type Boolean))
  (locals (FirstRoom :type "Room Object Reference") (FinalRoom :type "Room Object Reference"))
  (`|ExecutionSequence`
    (:`then_0`
      (bind _rooms (`DungeonGraph.GetAllRoomsFromData` (`self.Graph`) (`self.FirstRoom`)))
      (set `local.FirstRoom` (`|GetArrayItem` _rooms))
      (bind _rooms_2 (`DungeonGraph.GetAllRoomsFromData` (`self.Graph`) (`self.EndRoom`)))
      (set `local.FinalRoom` (`|GetArrayItem` _rooms_2)))
    (:`then_1`
      (bind (_resultpath _returnvalue) (`DungeonGraph.GetPathBetween` (`self.Graph`) (`local.FirstRoom`) (`local.FinalRoom`) false))
      (if _returnvalue
        (return (>= (`KismetArrayLibrary.Array_Length` _resultpath) (`self.MinLength`)))
        (else
          (return false))))))

(fn `RoomMeetsMaxCount`
  (params (RoomData :type "RoomData Object Reference"))
  (returns (Out :type Boolean))
  (locals (L_RoomData :type "/Game/Maps/Dungeon/Rooms/DungeonRoomData Object Reference"))
  (bind _asdungeon_room_data (cast `/Game/Maps/Dungeon/Rooms/DungeonRoomData` RoomData))
  (set `local.L_RoomData` _asdungeon_room_data)
  (if (> (`/Game/Maps/Dungeon/Rooms/DungeonRoomData.MaxCount` _asdungeon_room_data) 0)
    (bind _rooms (`DungeonGraph.GetAllRoomsFromData` (`self.Graph`) "/Game/Maps/Dungeon/Rooms/Test/RoomData_RoundStaircase.RoomData_RoundStaircase"))
    (return (< (`KismetArrayLibrary.Array_Length` _rooms) (`/Game/Maps/Dungeon/Rooms/DungeonRoomData.MaxCount` (`local.L_RoomData`))))
    (else
      (return true))))

(fn `SelectMobToSpawn`
  (returns (Mob :type "/Game/Blueprint/Entities/BP_Mob Class Reference"))
  (locals (Mobs :type "Array of /Game/Blueprint/Entities/BP_Mob Class Reference"))
  (bind _outitem (`KismetArrayLibrary.Array_Random` (`local.Mobs`)))
  (bind _outrownames (`DataTableFunctionLibrary.GetDataTableRowNames` "/Game/Data/DT_MobSpawnTable.DT_MobSpawnTable"))
  (for _array_element _outrownames
    (bind _returnvalue (`|GetDataTableRow` "/Game/Data/DT_MobSpawnTable.DT_MobSpawnTable" _array_element)
      (:`then`
        (bind (_mobclass _weight) (break `/Game/Data/Struct_MobSpawnData` _returnvalue))
        (for _ (range (+ _weight 1))
          (`KismetArrayLibrary.Array_Add` (`local.Mobs`) _mobclass)))))
  (`KismetSystemLibrary.PrintString` (`KismetSystemLibrary.GetClassDisplayName` _outitem))
  (return _outitem))

(fn `SetupQuest`
  (bind _asgm_main (cast `/Game/Blueprint/GM_Main` (`GameplayStatics.GetGameMode`)))
  (bind _success (`/Game/Blueprint/Quests/BP_Quest.SetupQuest` (`/Game/Blueprint/GM_Main.Quest` _asgm_main) (`self.Graph`)))
  (`KismetSystemLibrary.PrintString` (`KismetMathLibrary.SelectString` "Quest setup successful" "Quest setup failed" _success)))

(fn `SpawnCreatures`
  (bind _outactors (`GameplayStatics.GetAllActorsOfClassWithTag` "/Game/Blueprint/BP_SpawnPoint.BP_SpawnPoint_C" "Mob"))
  (for _array_element _outactors
    (bind _mob (`self.SelectMobToSpawn`))
    (bind _returnvalue_location (`KismetMathLibrary.BreakTransform` (`self.GetTransform` _array_element)))
    (`|SpawnActorFromClass` _mob (`KismetMathLibrary.MakeTransform` (+ _returnvalue_location (0.0 0.0 50.0))) "AdjustIfPossibleButAlwaysSpawn" "MultiplyWithRoot" null null)))

(fn `SpawnTraps`
  (bind _outactors (`GameplayStatics.GetAllActorsOfClassWithTag` "/Game/Blueprint/BP_SpawnPoint.BP_SpawnPoint_C" "Trap"))
  (for _array_element _outactors
    (`|SpawnActorFromClass` "/Game/Blueprint/Trap/TeleportationCircle/BP_Portal.BP_Portal_C" (`KismetMathLibrary.MakeTransform` (`self.K2_GetActorLocation` _array_element)) "Undefined" "MultiplyWithRoot" _array_element null)))

(fn `UserConstructionScript`)