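; Player state for adventurers that sets up proximity voice chat and shows a session debug widget for the local player.
; On BeginPlay it adds a VOIP Talker, registers it with itself after a short delay, and lowers the mic threshold.
; With a valid player controller, it attaches the voice to the controlled pawn's root using proximity attenuation.
; For the local controller, console commands turn on speaking and raise mic gain.
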(event `self.ReceiveBeginPlay`
  (bind _returnvalue (`self.GetPlayerController`))
  (`self.Initialize Proximity Chat`)
  (`/Engine/EditorBlueprintResources/StandardMacros.IsValid` _returnvalue
    (:`Is Valid`
      (if (`Controller.IsLocalPlayerController` _returnvalue)
        (bind _returnvalue_2 (`|CreateWidget` "/Game/Blueprint/WB_sessionDebug.WB_sessionDebug_C" _returnvalue))
        (`/Engine/EditorBlueprintResources/StandardMacros.IsValid` _returnvalue_2
          (:`Is Valid`
            (`UserWidget.AddToViewport` _returnvalue_2 0)))))))

(event `Initialize Proximity Chat`
  (bind _returnvalue (`self.GetPlayerController`))
  (bind _returnvalue_2 (`AddComponent|NODE_AddVOIPTalker-1`))
  (set `self.ref_VOIP` _returnvalue_2)
  (`KismetSystemLibrary.Delay` 0.2)
  (`VOIPTalker.RegisterWithPlayerState` (`self.ref_VOIP`) self)
  (`VOIPStatics.SetMicThreshold` -1.0)
  (`/Engine/EditorBlueprintResources/StandardMacros.IsValid` _returnvalue
    (:`Is Valid`
      (set `VOIPTalker.Settings` (make `VoiceSettings` (`Actor.RootComponent` (`Controller.K2_GetPawn` _returnvalue)) "/Game/Players/SA_ProximityVoice.SA_ProximityVoice") (`self.ref_VOIP`))
      (if (`Controller.IsLocalPlayerController` (`self.GetPlayerController`))
        (`KismetSystemLibrary.ExecuteConsoleCommand` "ToggleSpeaking 1" null)
        (`KismetSystemLibrary.ExecuteConsoleCommand` "voice.MicInputGain 6" null)))))

(fn `UserConstructionScript`)