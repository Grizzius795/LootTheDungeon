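; BP_Adventurer is the player character, handling movement, aiming, jumping and a visible carried-item inventory.
; Picked-up items enter BPC_Inventory, attach to hip or back slots using item-data offsets, and become held.
; Four item inputs tuck the current item and move the selected one to the right hand; dropping detaches it and clears its slot.
; Item changes route through S_ (server-prefixed) wrapper events before the local attach logic.
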(event `self.ReceiveBeginPlay`)

(event `/Game/Players/BPI_Controls.CharacterMove`
  (params (x :type "Float (double-precision)") (y :type "Float (double-precision)"))
  (`self.PlayerMove` x y))

(event `/Game/Players/BPI_Controls.CharacterAim`
  (params (Yaw :type "Float (double-precision)") (Pitch :type "Float (double-precision)"))
  (`self.PlayerAim` Yaw Pitch))

(event `/Game/Players/BPI_Controls.CharacterJump`
  (`self.Jump`))

(event `self.BPC_Inventory.OnSetItemInSlot`
  (params (SlotID :type Integer) (Item :type Name))
  (`self.Server_AddItemInSlot` SlotID Item))

(event `Server_AddItemInSlot`
  (params (SlotID :type Integer) (Item :type Name))
  (`self.Client_AddItemInSlot` SlotID Item))

(event `Client_AddItemInSlot`
  (params (`Slot ID` :type Integer) (Item :type Name))
  (`self.AttachItemToBeltSlot` null `Slot ID`))

(event `/Game/Players/BPI_Controls.DropItem`
  (`self.S_DropHeldItem`))

(event `S_DropHeldItem`
  (`self.DropHeldItem`))

(event `EnhancedInput|/Game/Input/Actions/IA_Item1`
  (params (ActionValue :type Boolean) (ElapsedSeconds :type "Float (double-precision)") (TriggeredSeconds :type "Float (double-precision)") (InputAction :type "InputAction Object Reference" :default "/Game/Input/Actions/IA_Item1.IA_Item1"))
  (:`Triggered`
    (`self.S_SetHeldItem` 0)))

(event `EnhancedInput|/Game/Input/Actions/IA_Item2`
  (params (ActionValue :type Boolean) (ElapsedSeconds :type "Float (double-precision)") (TriggeredSeconds :type "Float (double-precision)") (InputAction :type "InputAction Object Reference" :default "/Game/Input/Actions/IA_Item2.IA_Item2"))
  (:`Triggered`
    (`self.S_SetHeldItem` 1)))

(event `DropHeldItem`
  (`self.DropRightHandWeapon`))

(event `EnhancedInput|/Game/Input/Actions/IA_Item3`
  (params (ActionValue :type Boolean) (ElapsedSeconds :type "Float (double-precision)") (TriggeredSeconds :type "Float (double-precision)") (InputAction :type "InputAction Object Reference" :default "/Game/Input/Actions/IA_Item3.IA_Item3"))
  (:`Triggered`
    (`self.S_SetHeldItem` 2)))

(event `EnhancedInput|/Game/Input/Actions/IA_Item4`
  (params (ActionValue :type Boolean) (ElapsedSeconds :type "Float (double-precision)") (TriggeredSeconds :type "Float (double-precision)") (InputAction :type "InputAction Object Reference" :default "/Game/Input/Actions/IA_Item4.IA_Item4"))
  (:`Triggered`
    (`self.S_SetHeldItem` 3)))

(event `S_SetHeldItem`
  (params (SlotID :type Integer))
  (`self.SetHeldItem` SlotID))

(event `SetHeldItem`
  (params (SlotID :type Integer))
  (`self.SetRightHandItem` SlotID))

(event `/Game/Items/BPI_Items.Pick Up Item`
  (params (ref_item :type "/Game/Items/BP_Item Object Reference"))
  (bind (_itemslotid _bsuccess) (`/Game/Players/BPC_Inventory.AddItem` (`self.BPC_Inventory`) (`/Game/Items/BP_Item.Item` ref_item)))
  (if _bsuccess
    (`self.S_AddItemToBelt` ref_item _itemslotid)
    (`self.S_SetHeldItem` _itemslotid)))

(event `S_AddItemToBelt`
  (params (Item :type "/Game/Items/BP_Item Object Reference") (SlotID :type Integer))
  (`self.AddItemToBelt` Item SlotID))

(event `AddItemToBelt`
  (params (Item :type "/Game/Items/BP_Item Object Reference") (SlotID :type Integer))
  (`self.AttachItemToBeltSlot` Item SlotID))

(fn `AttachItemToBeltSlot`
  (params (Item :type "/Game/Items/BP_Item Object Reference") (SlotID :type Integer))
  (bind _item (`local.Item`))
  (bind ((`BeltSlotType_17_840896F0420D84B553400490E2CC648E` _beltslottype) (`Belt_LocationOffset_23_1A8AB9E641921EDA468372BDF5C9E520` _belt_locationoffset) (`Belt_rotationOffset_24_5F4812224C68E5549C7A53AE668686FE` _belt_rotationoffset)) (break `/Game/Items/Struct_Item` (`/Game/Items/BPFL_Items.GetItemData` (`/Game/Items/BP_Item.Item` Item))))
  (`/Engine/EditorBlueprintResources/StandardMacros.IsValid` Item
    (:`Is Valid`
      (`|ExecutionSequence`
        (:`then_0`
          (`/Game/Items/BP_Item.AttachToComponent` _item (select `/Game/Items/Enum_BeltSlotType` _beltslottype :`NewEnumerator0` (select `int` (`local.SlotID`) :`0` (`self.BeltSlot1`) :`1` (`self.BeltSlot2`) :`2` (`self.BeltSlot3`) :`3` (`self.BeltSlot4`) :!type "SceneComponent Object Reference") :`NewEnumerator1` (select `int` (`local.SlotID`) :`0` (`self.BackSlot1`) :`1` (`self.BackSlot2`) :`2` (`self.BackSlot3`) :`3` (`self.BackSlot4`) :!type "SceneComponent Object Reference")))
          (`self.K2_SetActorRelativeTransform` _item (`KismetMathLibrary.MakeTransform` _belt_locationoffset _belt_rotationoffset) false false))
        (:`then_1`
          (`KismetArrayLibrary.Array_Set` (`self.BeltItems`) (`local.SlotID`) (`local.Item`)))))))

(fn `DropRightHandWeapon`
  (bind _ref_righthanditem (`self.ref_RightHandItem`))
  (`/Engine/EditorBlueprintResources/StandardMacros.IsValid` _ref_righthanditem
    (:`Is Valid`
      (`/Game/Items/BP_Item.DetachFromParent` _ref_righthanditem)
      (set `self.ref_RightHandItem` null)
      (`/Game/Players/BPC_Inventory.SetItemInSlot` (`self.BPC_Inventory`) "None" (`self.RightHandItemSlot`))
      (`KismetArrayLibrary.Array_Set` (`self.BeltItems`) (`self.RightHandItemSlot`))
      (set `self.RightHandItemSlot` -1)
      (`self.OnSetHeldItem`))))

(fn `GetViewLocation`
  (returns (`View location` :type "Vector Structure") (`View Vector` :type "Vector Structure"))
  (bind _camera (`self.Camera`))
  (return (`SceneComponent.K2_GetComponentLocation` _camera) (`SceneComponent.GetForwardVector` _camera)))

(fn `PlayerAim`
  (params (Yaw :type "Float (double-precision)") (Pitch :type "Float (double-precision)"))
  (`self.AddControllerPitchInput` Pitch)
  (`self.AddControllerYawInput` Yaw))

(fn `PlayerMove`
  (params (`left / right` :type "Float (double-precision)") (`forward / backward` :type "Float (double-precision)"))
  (`self.AddMovementInput` (`self.GetActorRightVector`) `left / right`)
  (`self.AddMovementInput` (`self.GetActorForwardVector`) `forward / backward`))

(fn `SetRightHandItem`
  (params (`Slot ID` :type Integer))
  (`|ExecutionSequence`
    (:`then_0`
      (`self.TuckRightHandItem`))
    (:`then_1`
      (bind _output_get (set `self.RightHandItemSlot` (`local.Slot ID`)))
      (bind _output (`|GetArrayItem` (`self.BeltItems`) _output_get))
      (`/Engine/EditorBlueprintResources/StandardMacros.IsValid` _output
        (:`Is Valid`
          (set `self.ref_RightHandItem` _output)
          (`/Game/Items/BP_Item.AttachToComponent` (`self.ref_RightHandItem`) (`self.RightHand`)))))
    (:`then_2`
      (`self.OnSetHeldItem`))))

(fn `TuckRightHandItem`
  (`|ExecutionSequence`
    (:`then_0`
      (`/Engine/EditorBlueprintResources/StandardMacros.IsValid` (`self.ref_RightHandItem`)
        (:`Is Valid`
          (`self.AttachItemToBeltSlot` (`self.ref_RightHandItem`) (`self.RightHandItemSlot`)))))
    (:`then_1`
      (set `self.ref_RightHandItem` null)
      (set `self.RightHandItemSlot` -1))))

(fn `UserConstructionScript`)