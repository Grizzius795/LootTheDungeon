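; Player inventory component that stores items in an array of slots, resized to a set size on BeginPlay.
; A slot counts as empty when its item resolves to invalid item data.
; AddItem places an item in the first empty slot and reports the slot index, or fails when full.
; All writes go through SetItemInSlot, which broadcasts the OnSetItemInSlot dispatcher with the slot and item.
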(event `self.ReceiveBeginPlay`
  (`KismetArrayLibrary.Array_Resize` (`self.items`) (`self.Size`)))

(fn `AddItem`
  (params (NewItem :type Name))
  (returns (ItemSlotID :type Integer) (bSuccess :type Boolean))
  (locals (EmptySlot :type Integer :default 0))
  (bind (_emptyslotid _bfoundslot) (`self.FindEmptySlot`))
  (if _bfoundslot
    (set `local.EmptySlot` _emptyslotid)
    (`self.SetItemInSlot` (`local.NewItem`) (`local.EmptySlot`))
    (return (`local.EmptySlot`) true)
    (else
      (return 0 false))))

(fn `FindEmptySlot`
  (returns (EmptySlotID :type Integer) (bFoundSlot :type Boolean))
  (for (_array_element _array_index) (`self.items`)
    (if (not (`.is valid` (`/Game/Items/BPFL_Items.GetItemData` _array_element)))
      (return _array_index true)))
  (return -1 false))

(fn `GetItemInSlot`
  (params (SlotID :type Integer))
  (returns (OutItem :type Name) (bIsValid :type Boolean))
  (bind _output (`|GetArrayItem` (`self.items`) SlotID))
  (return _output (`.is valid` (`/Game/Items/BPFL_Items.GetItemData` _output))))

(fn `SetItemInSlot`
  (params (Item :type Name) (Slot :type Integer))
  (`KismetArrayLibrary.Array_Set` (`self.items`) Slot Item)
  (`self.OnSetItemInSlot` (`local.Slot`) (`local.Item`)))