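; BP_Spectator is a spectator that follows an adventurer player's character once it is possessed.
; On possession it passes the first BP_AdventurerController found to SetTarget, which stores that controller's BP_Adventurer pawn and attaches itself to it, snapping location and keeping world rotation and scale.
; After a short delay it calls SetInput on its own adventurer controller.
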(event `self.ReceivePossessed`
  (params (NewController :type "Controller Object Reference"))
  (bind _outactors (`GameplayStatics.GetAllActorsOfClass` "/Game/Blueprint/Players/BP_AdventurerController.BP_AdventurerController_C"))
  (`self.SetTarget` (`|GetArrayItem` _outactors))
  (`KismetSystemLibrary.Delay` 0.2)
  (bind _asbp_adventurer_controller (cast `/Game/Blueprint/Players/BP_AdventurerController` (`self.GetController`)))
  (`/Game/Blueprint/Players/BP_AdventurerController.Set Input` _asbp_adventurer_controller))

(fn `SetTarget`
  (params (`New SpecTarget` :type "/Game/Blueprint/Players/BP_AdventurerController Object Reference"))
  (bind _asbp_adventurer (cast `/Game/Blueprint/Players/BP_Adventurer` (`Controller.K2_GetPawn` `New SpecTarget`)))
  (set `self.SpecTarget` _asbp_adventurer)
  (`self.K2_AttachToActor` self (`self.SpecTarget`) "None" "SnapToTarget" "KeepWorld" "KeepWorld" true))

(fn `UserConstructionScript`)