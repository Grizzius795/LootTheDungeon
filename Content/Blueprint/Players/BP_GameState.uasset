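; BP_GameState is a game state Blueprint that drives the loading screen and biome card UI.
; Each action pairs an S_-prefixed entry event with a second event that does the widget work.
; Starting loading creates, stores and displays WB_Loading, and ending it calls FinishLoading on that stored widget.
; Showing the biome card creates a new WB_BiomeCard and adds it to the viewport without keeping a reference.
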(event `S_StartLoadingScreen`
  (`self.StartloadingScreen`))

(event `StartloadingScreen`
  (bind _returnvalue (`|CreateWidget` "/Game/Widgets/LoadingScreen/WB_Loading.WB_Loading_C"))
  (bind _output_get (set `self.LoadingScreen` _returnvalue))
  (`UserWidget.AddToViewport` _output_get 0))

(event `S_EndLoadingScreen`
  (`self.EndLoadingScreen`))

(event `EndLoadingScreen`
  (`/Game/Widgets/LoadingScreen/WB_Loading.FinishLoading` (`self.LoadingScreen`)))

(event `S_ShowBiomeCard`
  (`self.ShowBiomeCard`))

(event `ShowBiomeCard`
  (bind _returnvalue (`|CreateWidget` "/Game/Widgets/BiomeCard/WB_BiomeCard.WB_BiomeCard_C"))
  (`UserWidget.AddToViewport` _returnvalue 0))

(fn `UserConstructionScript`)