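; Player stamina component that stores stamina as an array of segmented bars, created full at BeginPlay, with functions to add, remove and check them.
; Spending drains the first non-empty bar without carrying overflow, then sets a looping timer with an initial delay for recovery.
; Recovery refills the last non-full bar, so bars refill in reverse order of draining.
; Both spending and recovery broadcast OnModifyStamina with the bar index and value.
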(event `self.ReceiveBeginPlay`
  (for _ (range (`self.BarsAmount`))
    (`self.AddStaminaBar` true)))

(event `SetStaminaRecoveryTimer`
  (`KismetSystemLibrary.K2_SetTimerDelegate` (`|CreateDelegate` :!event `BeginStaminaRecovery`) 0.1 true false (`self.StaminaRecoveryDelay`)))

(event `BeginStaminaRecovery`
  (`self.RecoverStamina` (`self.StaminaRecoveryRate`)))

(fn `AddStaminaBar`
  (params (AddFull :type Boolean))
  (`KismetArrayLibrary.Array_Add` (`self.StaminaBars`) (`KismetMathLibrary.SelectInt` (`self.StaminaPerBar`) 0 AddFull)))

(fn `IsStaminaEmpty`
  (returns (Empty :type Boolean))
  (locals (NotEmpty :type Boolean))
  (for _array_element (`self.StaminaBars`)
    (if (not (<= _array_element 0))
      (set `local.NotEmpty` true)))
  (return (not (`local.NotEmpty`))))

(fn `RecoverStamina`
  (params (Amount :type Integer))
  (locals (bar :type Integer) (Bars :type "Array of Integer") (bDone :type Boolean))
  (bind _bar (`local.bar`))
  (bind (_arrayindex _arrayelement) (`/Engine/EditorBlueprintResources/StandardMacros.ReverseForEachLoop` (`self.StaminaBars`))
    (:`LoopBody`
      (if (`local.bDone`)
        _
        (elif (< _arrayelement (`self.StaminaPerBar`))
          (set `local.bar` _arrayindex)
          (`KismetArrayLibrary.Array_Set` (`self.StaminaBars`) _arrayindex (`KismetMathLibrary.Clamp` (+ (`|GetArrayItem` (`self.StaminaBars`) _arrayindex) (`local.Amount`)) 0 (`self.StaminaPerBar`)))
          (set `local.bDone` true))))
    (:`Completed`
      (`self.OnModifyStamina` _bar (`|GetArrayItem` (`self.StaminaBars`) _bar)))))

(fn `RemoveStaminaBar`
  (`KismetArrayLibrary.Array_Remove` (`self.StaminaBars`)))

(fn `SpendStamina`
  (params (Amount :type Integer))
  (locals (DrainedBar :type Integer))
  (for (_array_element _array_index) (`self.StaminaBars`)
    (if (> _array_element 0)
      (set `local.DrainedBar` _array_index)
      (`KismetArrayLibrary.Array_Set` (`self.StaminaBars`) (`local.DrainedBar`) (`KismetMathLibrary.Clamp` (- (`|GetArrayItem` (`self.StaminaBars`) _array_index) (`local.Amount`)) 0 (`self.StaminaPerBar`)))
      (break)))
  (`self.OnModifyStamina` (`local.DrainedBar`) (`|GetArrayItem` (`self.StaminaBars`) (`local.DrainedBar`)))
  (`self.SetStaminaRecoveryTimer`))