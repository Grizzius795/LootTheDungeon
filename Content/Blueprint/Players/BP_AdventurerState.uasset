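; Player state for adventurers that owns the player's saved character customization and background music switching.
; On BeginPlay it polls until a pawn exists, loads the "CustomCharacter" save or creates a randomized one, then registers the customization with GM_Main.
; PlayBGM runs one volume timeline, swaps the track, then runs a second, and SaveCustomization writes the data back to the slot.
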(event `self.ReceiveBeginPlay`
  (`/Engine/EditorBlueprintResources/StandardMacros.IsValid` (`self.GetPawn`) :!label _label
    (:`Is Valid`
      (`|ExecutionSequence`
        (:`then_0`
          (bind _returnvalue (`GameplayStatics.DoesSaveGameExist` "CustomCharacter"))
          (if _returnvalue
            (bind _returnvalue_2 (`GameplayStatics.LoadGameFromSlot` "CustomCharacter"))
            (bind _asbp_save_character (cast `/Game/Blueprint/Save/BP_SaveCharacter` _returnvalue_2))
            (set `self.CustomCharacterData` _asbp_save_character)
            (else
              (bind _returnvalue_3 (`GameplayStatics.CreateSaveGameObject` "/Game/Blueprint/Save/BP_SaveCharacter.BP_SaveCharacter_C"))
              (bind _output_get (set `self.CustomCharacterData` _returnvalue_3))
              (`/Game/Blueprint/Save/BP_SaveCharacter.Random` _output_get))))
        (:`then_1`
          (bind _asgm_main (cast `/Game/Blueprint/GM_Main` (`GameplayStatics.GetGameMode`)))
          (`/Game/Blueprint/GM_Main.AddPlayerCustomization` _asgm_main self (`/Game/Blueprint/Save/BP_SaveCharacter.Customization` (`self.CustomCharacterData`))))))
    (:`Is Not Valid`
      (`KismetSystemLibrary.Delay` 0.2)
      (goto _label))))

(event `PlayBGM`
  (params (`New track` :type "SoundCue Object Reference"))
  (bind _track_bgm (`self.Track_BGM`))
  (bind (_direction _newtrack_0) (`Timeline|Timeline_0` :!via `PlayFromStart`)
    (:`Update`
      (`AudioComponent.SetVolumeMultiplier` (`self.Track_BGM`) _newtrack_0))
    (:`Finished`
      (`AudioComponent.SetSound` _track_bgm `New track`)
      (`AudioComponent.Play` _track_bgm 0.0)
      (bind (_direction_2 _newtrack_0_2) (`Timeline|Timeline` :!via `PlayFromStart`)
        (:`Update`
          (`AudioComponent.SetVolumeMultiplier` (`self.Track_BGM`) _newtrack_0_2))))))

(event `SaveCustomization`
  (`GameplayStatics.SaveGameToSlot` (`self.CustomCharacterData`) "CustomCharacter"))

(fn `UserConstructionScript`)