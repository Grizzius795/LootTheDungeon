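; Multiplayer first-person player character with Steam name tags, proximity voice chat and saved skin color.
; Input and gameplay events relay through S_ events for movement, belt inventory, held-item use and interaction.
; Components drive stamina-limited sprint and jump, health, and physical-animation ragdoll, while held items or an unarmed sphere deal strike damage.
; Death dissolves the mesh into a skeleton, then possesses a spectator; name tags show only within unobstructed range.
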(event `SetDisplayNameRotation`
  (bind _returnvalue (`Controller.K2_GetPawn` (`GameplayStatics.GetPlayerController` 0)))
  (bind _view_location (message `/Game/Blueprint/Players/BPI_Controls.GetViewLocation` _returnvalue))
  (bind _outhit (`KismetSystemLibrary.LineTraceSingle` _view_location (`SceneComponent.K2_GetComponentLocation` (`self.Widget`)) "TraceTypeQuery1" false (`|MakeArray` _returnvalue :!type "Actor Object Reference")))
  (bind (_bblockinghit _binitialoverlap _time _distance _location _impactpoint _normal _impactnormal _physmat _hitactor _hitcomponent _hitbonename _bonename _hititem _elementindex _faceindex _tracestart _traceend) (`GameplayStatics.BreakHitResult` _outhit))
  (`SceneComponent.SetVisibility` (`self.Widget`) (and (not _bblockinghit) (< (`KismetMathLibrary.Vector_Distance` _tracestart _traceend) 1500.0)) false))

(event `S_InitializeProximityChat`
  (`self.InitializeProximityChat`))

(event `InitializeProximityChat`
  (bind _returnvalue (`self.GetController`))
  (bind _returnvalue_2 (`AddComponent|NODE_AddVOIPTalker-1`))
  (set `self.ref_VOIP` _returnvalue_2)
  (`/Engine/EditorBlueprintResources/StandardMacros.IsValid` (`self.PlayerState`) :!label _label
    (:`Is Valid`
      (`VOIPTalker.RegisterWithPlayerState` (`self.ref_VOIP`) (`self.PlayerState`))
      (`VOIPStatics.SetMicThreshold` -1.0)
      (set `VOIPTalker.Settings` (make `VoiceSettings` (`self.Camera`) "/Game/Blueprint/Players/SA_ProximityVoice.SA_ProximityVoice") (`self.ref_VOIP`))
      (`/Engine/EditorBlueprintResources/StandardMacros.IsValid` _returnvalue
        (:`Is Valid`
          (if (`Controller.IsLocalPlayerController` _returnvalue)
            (bind _asplayer_controller (cast `PlayerController` _returnvalue))
            (`KismetSystemLibrary.ExecuteConsoleCommand` "ToggleSpeaking 1" _asplayer_controller)))))
    (:`Is Not Valid`
      (`KismetSystemLibrary.Delay` 1.0)
      (goto _label))))

(event `self.ReceiveTick`
  (params (DeltaSeconds :type "Float (single-precision)"))
  (`self.SetDisplayNameRotation`))

(event `/Game/Blueprint/Players/BPI_Controls.CharacterMove`
  (params (x :type "Float (double-precision)") (y :type "Float (double-precision)"))
  (`self.PlayerMove` x y))

(event `self.ReceiveBeginPlay`
  (bind _returnvalue (`self.GetController`))
  (`|ExecutionSequence`
    (:`then_0`
      (bind _aswb_display_name (cast `/Game/Blueprint/Players/HUD/WB_DisplayName` (`WidgetComponent.GetWidget` (`self.Widget`))))
      (`/Engine/EditorBlueprintResources/StandardMacros.IsValid` _returnvalue
        (:`Is Valid`
          (bind _returnvalue_2 (`AdvancedSteamFriendsLibrary.GetSteamPersonaName` (`AdvancedSessionsLibrary.GetUniqueNetIDFromPlayerState` (`Controller.PlayerState` _returnvalue))))
          (`/Game/Blueprint/Players/HUD/WB_DisplayName.SetName` _aswb_display_name _returnvalue_2))
        (:`Is Not Valid`
          (`/Game/Blueprint/Players/HUD/WB_DisplayName.SetName` _aswb_display_name ""))))
    (:`then_1`
      (`self.S_InitializeProximityChat`)
      (bind _returnvalue_3 (`|CreateWidget` "/Game/Blueprint/Players/HUD/WB_PlayerHUD.WB_PlayerHUD_C"))
      (`UserWidget.AddToViewport` _returnvalue_3 0)
      (bind _asbp_adventurer_controller (cast `/Game/Blueprint/Players/BP_AdventurerController` (`self.GetController`)))
      (set `/Game/Blueprint/Players/BP_AdventurerController.HUD` _returnvalue_3 _asbp_adventurer_controller))
    (:`then_2`
      (set `SceneCaptureComponent.ShowOnlyActors` (`|MakeArray` self :!type "Actor Object Reference") (`self.SceneCaptureComponent2D`))
      (`self.S_InitAppearance`))))

(event `/Game/Blueprint/Players/BPI_Controls.CharacterAim`
  (params (Yaw :type "Float (double-precision)") (Pitch :type "Float (double-precision)"))
  (`self.PlayerAim` Yaw Pitch))

(event `/Game/Blueprint/Players/BPI_Controls.CharacterJump`
  (if (and (`NavMovementInterface.IsMovingOnGround` (`self.CharacterMovement`)) (not (`/Game/Blueprint/Players/BPC_Stamina.IsStaminaEmpty` (`self.BPC_Stamina`))))
    (`self.Jump`)
    (`/Game/Blueprint/Players/BPC_Stamina.SpendStamina` (`self.BPC_Stamina`) 12)))

(event `self.BPC_Inventory.OnSetItemInSlot`
  (params (SlotID :type Integer) (Item :type "/Game/Blueprint/Items/BP_Item Object Reference"))
  (`self.Server_AddItemInSlot` SlotID Item))

(event `Server_AddItemInSlot`
  (params (SlotID :type Integer) (Item :type "/Game/Blueprint/Items/BP_Item Object Reference"))
  (`self.Client_AddItemInSlot` SlotID Item))

(event `Client_AddItemInSlot`
  (params (`Slot ID` :type Integer) (Item :type "/Game/Blueprint/Items/BP_Item Object Reference"))
  (`self.AttachItemToBeltSlot` Item `Slot ID`))

(event `/Game/Blueprint/Players/BPI_Controls.DropItem`
  (`self.S_DropHeldItem`))

(event `S_DropHeldItem`
  (`self.DropHeldItem`))

(event `EnhancedInput|/Game/Input/Actions/IA_Item1`
  (params (ActionValue :type Boolean) (ElapsedSeconds :type "Float (double-precision)") (TriggeredSeconds :type "Float (double-precision)") (InputAction :type "InputAction Object Reference" :default "/Game/Input/Actions/IA_Item1.IA_Item1"))
  (:`Started`
    (`self.S_SetHeldItem` 0)))

(event `EnhancedInput|/Game/Input/Actions/IA_Item2`
  (params (ActionValue :type Boolean) (ElapsedSeconds :type "Float (double-precision)") (TriggeredSeconds :type "Float (double-precision)") (InputAction :type "InputAction Object Reference" :default "/Game/Input/Actions/IA_Item2.IA_Item2"))
  (:`Started`
    (`self.S_SetHeldItem` 1)))

(event `DropHeldItem`
  (`self.DropRightHandWeapon`))

(event `EnhancedInput|/Game/Input/Actions/IA_Item3`
  (params (ActionValue :type Boolean) (ElapsedSeconds :type "Float (double-precision)") (TriggeredSeconds :type "Float (double-precision)") (InputAction :type "InputAction Object Reference" :default "/Game/Input/Actions/IA_Item3.IA_Item3"))
  (:`Started`
    (`self.S_SetHeldItem` 2)))

(event `EnhancedInput|/Game/Input/Actions/IA_Item4`
  (params (ActionValue :type Boolean) (ElapsedSeconds :type "Float (double-precision)") (TriggeredSeconds :type "Float (double-precision)") (InputAction :type "InputAction Object Reference" :default "/Game/Input/Actions/IA_Item4.IA_Item4"))
  (:`Started`
    (`self.S_SetHeldItem` 3)))

(event `S_SetHeldItem`
  (params (SlotID :type Integer))
  (`self.SetHeldItem` SlotID))

(event `SetHeldItem`
  (params (SlotID :type Integer))
  (`self.SetRightHandItem` SlotID))

(event `/Game/Blueprint/Items/BPI_Items.Pick Up Item`
  (params (ref_item :type "/Game/Blueprint/Items/BP_Item Object Reference"))
  (bind (_itemslotid _bsuccess) (`/Game/Blueprint/Players/BPC_Inventory.AddItem` (`self.BPC_Inventory`) ref_item))
  (if _bsuccess
    (`self.S_AddItemToBelt` ref_item _itemslotid)
    (`self.S_SetHeldItem` _itemslotid)))

(event `S_AddItemToBelt`
  (params (Item :type "/Game/Blueprint/Items/BP_Item Object Reference") (SlotID :type Integer))
  (`self.AddItemToBelt` Item SlotID))

(event `AddItemToBelt`
  (params (Item :type "/Game/Blueprint/Items/BP_Item Object Reference") (SlotID :type Integer))
  (`self.AttachItemToBeltSlot` Item SlotID))

(event `SetPOVItem`
  (`/Game/Blueprint/Items/BP_Item.AttachToComponent` (`self.ref_RightHandItem`) (`self.POV_RightHandItem`)))

(event `/Game/Blueprint/Players/BPI_Controls.ReleasePrimaryFire`
  ; item Use
  (`self.S_UsePrimaryFire`))

(event `/Game/Blueprint/Players/BPI_Attacks.BeginStrike`
  (bind _ref_righthanditem (`self.ref_RightHandItem`)
    (:`then`
      (message `/Game/Blueprint/Players/BPI_Attacks.BeginStrike` _ref_righthanditem))
    (:`else`
      (`PrimitiveComponent.SetCollisionEnabled` (`self.Sphere`) "QueryOnly"))))

(event `S_UsePrimaryFire`
  ; item Use
  (`self.UsePrimaryFire`))

(event `UsePrimaryFire`
  ; item Use
  (set `self.bHoldPrimary` false)
  (bind _ref_righthanditem (`self.ref_RightHandItem`)
    (:`then`
      (`/Game/Blueprint/Items/BP_Item.ReleasePrimaryUse` _ref_righthanditem))
    (:`else`)))

(event `/Game/Blueprint/Players/BPI_Attacks.FinishStrike`
  (bind _ref_righthanditem (`self.ref_RightHandItem`)
    (:`then`
      (message `/Game/Blueprint/Players/BPI_Attacks.FinishStrike` _ref_righthanditem))
    (:`else`
      (`PrimitiveComponent.SetCollisionEnabled` (`self.Sphere`) "NoCollision"))))

(event `self.BPC_Health.OnUnconscious`
  (`/Game/Blueprint/Players/BPI_Attacks.Ragdoll` (0.0 0.0 0.0)))

(event `/Game/Blueprint/Players/BPI_Controls.HoldPrimary`
  ; item Use
  (`self.S_HoldPrimaryFire`))

(event `S_HoldPrimaryFire`
  ; item Use
  (`self.HoldPrimaryFire`))

(event `HoldPrimaryFire`
  ; item Use
  (set `self.bHoldPrimary` true)
  (bind _ref_righthanditem (`self.ref_RightHandItem`)
    (:`then`
      (`/Game/Blueprint/Items/BP_Item.HoldPrimaryUse` _ref_righthanditem)
      ;;[0.8125 0.03722 0.2043 0.5] Commence le timer de l'attaque lourde
      (message `/Game/Blueprint/Players/BPI_Attacks.StartHoldingStrike` _ref_righthanditem))
    (:`else`)))

(event `/Game/Blueprint/Players/BPI_Attacks.Ragdoll`
  (params (`Ragdoll impulse` :type "Vector Structure"))
  ; Ragdoll
  (`self.Client_Ragdoll` `Ragdoll impulse`))

(event `Client_Ragdoll`
  (params (InputPin :type "Vector Structure"))
  ; Ragdoll
  (`self.SetReplicateMovement` true)
  (`KismetSystemLibrary.DelayUntilNextTick`)
  (`/Game/Blueprint/BPC_PhysicalAnim.EnterRagdoll` (`self.BPC_PhysicalAnim`))
  (`ActorComponent.Deactivate` (`self.Camera`))
  (`ActorComponent.Activate` (`self.CameraRagdoll`) false)
  (set `self.bUseControllerRotationYaw` false)
  (`PrimitiveComponent.AddImpulse` (`self.Mesh`) InputPin "None" false))

(event `GetUp`
  ; Ragdoll
  (`KismetSystemLibrary.DelayUntilNextTick`)
  (`/Game/Blueprint/BPC_PhysicalAnim.EndRagdoll` (`self.BPC_PhysicalAnim`))
  (`ActorComponent.Deactivate` (`self.CameraRagdoll`))
  (`ActorComponent.Activate` (`self.Camera`) false)
  (set `self.bUseControllerRotationYaw` true))

(event `S_GetUp`
  ; Ragdoll
  (`self.GetUp`))

(event `/Game/Blueprint/Players/BPI_Attacks.TakeHit`
  (params (HitInfo :type "/Game/Blueprint/Items/Struct_hitInfo Structure"))
  ; Ragdoll
  (`self.S_hitReaction` HitInfo))

(event `S_hitReaction`
  (params (HitInfo :type "/Game/Blueprint/Items/Struct_hitInfo Structure"))
  ; Ragdoll
  (`self.HitReaction` HitInfo))

(event `HitReaction`
  (params (HitInfo :type "/Game/Blueprint/Items/Struct_hitInfo Structure"))
  ; Ragdoll
  (`/Game/Blueprint/BPC_PhysicalAnim.HitReaction` (`self.BPC_PhysicalAnim`) HitInfo))

(event `self.OnRoomExit`
  (params (RoomLevel :type "RoomLevel Object Reference"))
  (if (== (`RoomLevel.GetRoomData` RoomLevel) "/Game/Maps/Dungeon/Rooms/LushLabyrinth/RoomData_LushStart.RoomData_LushStart")
    (`/Engine/EditorBlueprintResources/StandardMacros.DoOnce` false
      (:`Completed`
        (bind _asgm_main (cast `/Game/Blueprint/GM_Main` (`GameplayStatics.GetGameMode`)))
        (`/Game/Blueprint/GM_Main.ShowBiomeTitleCard` _asgm_main)))))

(event `EnhancedInput|/Game/Input/Actions/IA_Sprint`
  (params (ActionValue :type Boolean) (ElapsedSeconds :type "Float (double-precision)") (TriggeredSeconds :type "Float (double-precision)") (InputAction :type "InputAction Object Reference" :default "/Game/Input/Actions/IA_Sprint.IA_Sprint"))
  ; Sprint
  (:`Started`
    (`self.S_ToggleSprint` true))
  (:`Canceled`
    (`self.S_ToggleSprint` false :!label _label_2))
  (:`Completed`
    (goto _label_2)))

(event `S_ToggleSprint`
  (params (Condition :type Boolean))
  ; Sprint
  (`self.ToggleSprint` Condition))

(event `ToggleSprint`
  (params (Condition :type Boolean))
  ; Sprint
  (`|ExecutionSequence`
    (:`then_0`
      (bind _output_get (set `self.bSprinting` Condition))
      (if _output_get
        (bind (_direction _newtrack_0) (`Timeline|Timeline` :!via `ReverseFromEnd` :!label _label_3)
          (:`Update`
            (set `CharacterMovementComponent.MaxWalkSpeed` (`KismetMathLibrary.MapRangeClamped` _newtrack_0 0.0 1.0 (`self.RunSpeed`) (`self.WalkSpeed`)) (`self.CharacterMovement`))))
        (else
          (goto _label_3 :!via `PlayFromStart`))))
    (:`then_1`
      (if (`self.bSprinting`)
        (bind _returnvalue (`KismetSystemLibrary.K2_SetTimerDelegate` (delegate `SpendSprintStamina`) 0.2 true))
        (set `self.SprintStaminaTimer` _returnvalue)
        (else
          (`KismetSystemLibrary.K2_ClearAndInvalidateTimerHandle` (`self.SprintStaminaTimer`)))))))

(event `/Game/Blueprint/Players/BPI_Controls.Interact`
  (params (Target :type "/Game/Blueprint/BPC_Interactible Object Reference"))
  ; Interaction
  (`self.S_succeedInteract` Target))

(event `S_succeedInteract`
  (params (Target :type "/Game/Blueprint/BPC_Interactible Object Reference"))
  ; Interaction
  (`self.SucceedInteract` Target))

(event `SpendSprintStamina`
  (bind _bpc_stamina (`self.BPC_Stamina`))
  ; Sprint
  (if (`NavMovementInterface.IsMovingOnGround` (`self.CharacterMovement`))
    (`/Game/Blueprint/Players/BPC_Stamina.SpendStamina` _bpc_stamina 1)
    (if (`/Game/Blueprint/Players/BPC_Stamina.IsStaminaEmpty` _bpc_stamina)
      (`self.S_ToggleSprint` false))))

(event `SucceedInteract`
  (params (Target :type "/Game/Blueprint/BPC_Interactible Object Reference"))
  ; Interaction
  (`/Game/Blueprint/BPC_Interactible.SucceedInteract` Target self))

(event `self.BPC_PhysicalAnim.OnRagdollStopMoving`
  (`self.S_GetUp`))

(event `self.BPC_Health.OnDeath`
  ; Death
  (`/Engine/EditorBlueprintResources/StandardMacros.DoOnce` false
    (:`Completed`
      (`KismetSystemLibrary.DelayUntilNextTick`)
      (`|ExecutionSequence`
        (:`then_0`
          (bind _returnvalue (`KismetMaterialLibrary.CreateDynamicMaterialInstance` "/Game/Materials/M_Dissolve.M_Dissolve"))
          (bind _output_get (set `self.DissolveMaterial` _returnvalue))
          (`PrimitiveComponent.SetMaterial` (`self.Mesh`) 0 _output_get))
        (:`then_1`
          (bind (_direction _dissolve) (`Timeline|Timeline_0` :!via `PlayFromStart`)
            (:`Update`
              (`MaterialInstanceDynamic.SetScalarParameterValue` (`self.DissolveMaterial`) "Dissolve" _dissolve))
            (:`Finished`
              (`KismetSystemLibrary.Delay` 1.0)
              (bind _returnvalue_2 (`|SpawnActorFromClass` "/Game/Blueprint/Players/BP_Spectator.BP_Spectator_C" (`KismetMathLibrary.MakeTransform` (0.0 0.0 0.0)) "Undefined" "MultiplyWithRoot" null null))
              (bind _asbp_adventurer_controller (cast `/Game/Blueprint/Players/BP_AdventurerController` (`self.GetController`)))
              (`Controller.Possess` _asbp_adventurer_controller _returnvalue_2))))
        (:`then_2`
          (`KismetSystemLibrary.Delay` 1.2)
          (`NiagaraFunctionLibrary.SpawnSystemAtLocation` "/Game/Blueprint/Entities/NG_DeathExplosion.NG_DeathExplosion" (`SceneComponent.GetSocketLocation` (`self.Mesh`) "Hips"))
          (`SceneComponent.SetVisibility` (`self.Skeleton`) true false)
          (`SceneComponent.SetVisibility` (`self.Mesh`) false false))))))

(event `self.Sphere.OnComponentBeginOverlap`
  (params (OverlappedComponent :type "PrimitiveComponent Object Reference") (OtherActor :type "Actor Object Reference") (OtherComp :type "PrimitiveComponent Object Reference") (OtherBodyIndex :type Integer) (bFromSweep :type Boolean) (SweepResult :type "HitResult Structure (by ref)"))
  (bind (_outhit _returnvalue) (`KismetSystemLibrary.SphereTraceSingle` (`SceneComponent.K2_GetComponentLocation` (`self.Sphere`)) (`SceneComponent.K2_GetComponentLocation` OverlappedComponent) 4.0 "TraceTypeQuery1"))
  (if _returnvalue
    (`self.HitEvent` (`.HitActor` (`GameplayStatics.BreakHitResult` _outhit)) _outhit)))

(event `HitEvent`
  (params (TargetActor :type "Actor Object Reference") (HitResult :type "HitResult Structure"))
  (bind _returnvalue (`self.GetComponentByClass` TargetActor "/Game/Blueprint/Damage/BPC_Health.BPC_Health_C"))
  (bind (_bblockinghit _binitialoverlap _time _distance _location _impactpoint _normal _impactnormal _physmat _hitactor _hitcomponent _hitbonename _bonename _hititem _elementindex _faceindex _tracestart _traceend) (`GameplayStatics.BreakHitResult` HitResult))
  (`/Engine/EditorBlueprintResources/StandardMacros.IsValid` TargetActor
    (:`Is Valid`
      (`/Engine/EditorBlueprintResources/StandardMacros.IsValid` _returnvalue
        (:`Is Valid`
          (`|ExecutionSequence`
            (:`then_0`
              (bind (_keypin _valuepin) (`|MapForEach` (`self.Damages`))
                (:`then`
                  (`/Game/Blueprint/Damage/BPC_Health.TakeDamage` _returnvalue _keypin _valuepin (make `/Game/Blueprint/Damage/Struct_DamageParam` :`strings` (`|MakeMap` "HitBoneName" (`KismetStringLibrary.Conv_NameToString` _hitbonename) :!type "Name") :`Vectors` (`|MakeMap` "HitLocation" _location "HitNormal" _impactnormal "HitDirection" (`KismetMathLibrary.Normal` (- _traceend _tracestart)) :!type "Name") :`Actors` (`|MakeMap` "Perpetrator" self :!type "Name" :!valuetype "Actor Object Reference"))))))
            (:`then_1`
              (`PrimitiveComponent.SetCollisionEnabled` (`self.Sphere`) "NoCollision"))))))))

(event `S_SetSkinColor`
  (params (Value :type "/Game/Blueprint/Mirror/Struct_SkinColors Structure"))
  (`self.SetSkinColor` Value))

(event `SetSkinColor`
  (params (Value :type "/Game/Blueprint/Mirror/Struct_SkinColors Structure"))
  (bind _returnvalue (`self.GetController`))
  (bind _dynamicskincolor (`self.DynamicSkinColor`))
  (`/Engine/EditorBlueprintResources/StandardMacros.IsValid` _dynamicskincolor
    (:`Is Valid`
      _)
    (:`Is Not Valid`
      (`self.InitAppearance`)))
  (`MaterialInstanceDynamic.SetVectorParameterValue` _dynamicskincolor "SkinColor" (`.Color_9_89E0BCBA42CDB7980F13198DFAD18CFE` (break `/Game/Blueprint/Mirror/Struct_SkinColors` Value)))
  (`/Engine/EditorBlueprintResources/StandardMacros.IsValid` _returnvalue
    (:`Is Valid`
      (if (`Controller.IsLocalPlayerController` _returnvalue)
        (set `/Game/Blueprint/Save/BP_SaveCharacter.Skin color` Value (`self.Save_Character`))
        (`self.SaveCustomCharacter`)))))

(event `S_InitAppearance`
  (`self.InitAppearance`))

(event `InitAppearance`
  (bind _returnvalue (`self.GetController`))
  (bind _returnvalue_2 (`PrimitiveComponent.CreateDynamicMaterialInstance` (`self.Mesh`) 0 "/Game/Blueprint/Players/FBX/M_Player.M_Player" "None"))
  (set `self.DynamicSkinColor` _returnvalue_2)
  (`/Engine/EditorBlueprintResources/StandardMacros.IsValid` _returnvalue
    (:`Is Valid`
      (if (`Controller.IsLocalPlayerController` _returnvalue)
        (bind _returnvalue_3 (`GameplayStatics.DoesSaveGameExist` "CustomCharacter"))
        (if _returnvalue_3
          (bind _returnvalue_4 (`GameplayStatics.LoadGameFromSlot` "CustomCharacter"))
          (bind _asbp_save_character (cast `/Game/Blueprint/Save/BP_SaveCharacter` _returnvalue_4))
          (set `self.Save_Character` _asbp_save_character)
          (else
            (bind _returnvalue_5 (`GameplayStatics.CreateSaveGameObject` "/Game/Blueprint/Save/BP_SaveCharacter.BP_SaveCharacter_C"))
            (bind _output_get (set `self.Save_Character` _returnvalue_5))
            (`/Game/Blueprint/Save/BP_SaveCharacter.Random` _output_get)))
        (`self.S_SetSkinColor` (`/Game/Blueprint/Save/BP_SaveCharacter.Skin color` (`self.Save_Character`)))))))

(fn `AttachItemToBeltSlot`
  (params (Item :type "/Game/Blueprint/Items/BP_Item Object Reference") (SlotID :type Integer))
  (bind _item (`local.Item`))
  (`/Engine/EditorBlueprintResources/StandardMacros.IsValid` Item
    (:`Is Valid`
      (`/Game/Blueprint/Items/BP_Item.AttachToComponent` _item (select `/Game/Blueprint/Items/Enum_BeltSlotType` "NewEnumerator0" :`NewEnumerator0` (select `int` (`local.SlotID`) :`0` (`self.BeltSlot1`) :`1` (`self.BeltSlot2`) :`2` (`self.BeltSlot3`) :`3` (`self.BeltSlot4`) :!type "SceneComponent Object Reference") :`NewEnumerator1` (select `int` (`local.SlotID`) :`0` (`self.BackSlot1`) :`1` (`self.BackSlot2`) :`2` (`self.BackSlot3`) :`3` (`self.BackSlot4`) :!type "SceneComponent Object Reference")))
      (`self.K2_SetActorRelativeTransform` _item (`/Game/Blueprint/Items/BP_Item.Belt_Offset` (`local.Item`)) false true))))

(fn `DropRightHandWeapon`
  (bind _ref_righthanditem (`self.ref_RightHandItem`))
  (bind _righthanditemslot (`self.RightHandItemSlot`))
  (`/Engine/EditorBlueprintResources/StandardMacros.IsValid` _ref_righthanditem
    (:`Is Valid`
      (`/Game/Blueprint/Items/BP_Item.DetachFromParent` _ref_righthanditem)
      (set `/Game/Blueprint/BPC_Interactible.bInteractible` true (`/Game/Blueprint/Items/BP_Item.BPC_Interactible` _ref_righthanditem))
      (set `self.ref_RightHandItem` null)
      (`/Game/Blueprint/Players/BPC_Inventory.SetItemInSlot` (`self.BPC_Inventory`) _righthanditemslot null)
      (`self.SetRightHandItem` _righthanditemslot)
      (set `self.RightHandItemSlot` -1)
      (`self.OnSetHeldItem`))))

(fn `GetViewLocation`
  (returns (`View location` :type "Vector Structure") (`View Vector` :type "Vector Structure"))
  (bind _camera (`self.Camera`))
  (return (`SceneComponent.K2_GetComponentLocation` _camera) (`SceneComponent.GetForwardVector` _camera)))

(fn `PlayerAim`
  (params (Yaw :type "Float (double-precision)") (Pitch :type "Float (double-precision)"))
  (`self.AddControllerPitchInput` Pitch)
  (`self.AddControllerYawInput` Yaw))

(fn `PlayerMove`
  (params (`left / right` :type "Float (double-precision)") (`forward / backward` :type "Float (double-precision)"))
  (`self.AddMovementInput` (`self.GetActorRightVector`) `left / right`)
  (`self.AddMovementInput` (`self.GetActorForwardVector`) `forward / backward`))

(fn `SaveCustomCharacter`
  (`GameplayStatics.SaveGameToSlot` (`self.Save_Character`) "CustomCharacter"))

(fn `SetRightHandItem`
  (params (`Slot ID` :type Integer))
  (bind _ref_righthanditem (`self.ref_RightHandItem`))
  (`|ExecutionSequence`
    (:`then_0`
      (`self.TuckRightHandItem`)
      (`SkeletalMeshComponent.SetAnimInstanceClass` (`self.Mesh`) "/Game/Blueprint/Players/FBX/ABP_Player_Default.ABP_Player_Default_C"))
    (:`then_1`
      (bind _output_get (set `self.RightHandItemSlot` (`local.Slot ID`)))
      (bind (_outitem _bisvalid) (`/Game/Blueprint/Players/BPC_Inventory.GetItemInSlot` (`self.BPC_Inventory`) _output_get))
      (if _bisvalid
        (set `self.ref_RightHandItem` _outitem)
        (`/Game/Blueprint/Items/BP_Item.AttachToComponent` _ref_righthanditem (`self.RightHand`))
        (`self.K2_SetActorRelativeTransform` _ref_righthanditem (`/Game/Blueprint/Items/BP_Item.Held_offset` _ref_righthanditem) false false)
        (`SkeletalMeshComponent.SetAnimInstanceClass` (`self.Mesh`) (`/Game/Blueprint/Items/BP_Item.Held_Animation` (`self.ref_RightHandItem`)))))
    (:`then_2`
      (`self.OnSetHeldItem`))))

(fn `TuckRightHandItem`
  (`|ExecutionSequence`
    (:`then_0`
      (`/Engine/EditorBlueprintResources/StandardMacros.IsValid` (`self.ref_RightHandItem`)
        (:`Is Valid`
          (`self.AttachItemToBeltSlot` (`self.ref_RightHandItem`) (`self.RightHandItemSlot`)))))
    (:`then_1`
      (set `self.ref_RightHandItem` null)
      (set `self.RightHandItemSlot` -1))))

(fn `UserConstructionScript`)