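; Player controller for the adventurer that routes Enhanced Input to the controlled pawn through interface messages and opens the menu.
; Mouse look applies saved sensitivity and axis inversion from the game instance.
; Each tick, a view-aligned sphere trace finds interactibles to highlight and preview in a widget.
; Holding interact accumulates progress to the target's delay before messaging the pawn; the controller also hooks pawn death and keeps a death flag.
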(event `S_SetDeathFlag`
  (`self.SetDeathFlag`))

(event `SetDeathFlag`
  (set `self.bIsDead` true))

(event `self.ReceiveBeginPlay`
  (bind _returnvalue (`self.GetComponentByClass` (`self.K2_GetPawn`) "/Game/Blueprint/Damage/BPC_Health.BPC_Health_C"))
  (if (`self.IsLocalController`)
    (bind _returnvalue_2 (`|CreateWidget` "/Game/Blueprint/Players/HUD/WB_InteractPreview.WB_InteractPreview_C"))
    (set `self.InteractPreview` _returnvalue_2)
    (`self.Set Input`)
    (`/Engine/EditorBlueprintResources/StandardMacros.IsValid` _returnvalue
      (:`Is Valid`
        (add `/Game/Blueprint/Damage/BPC_Health.OnDeath` _returnvalue (`|CreateDelegate` :!event `S_SetDeathFlag`))))))

(event `Set Input`
  (bind _returnvalue (subsystem `EnhancedInputLocalPlayerSubsystem`))
  (bind _returnvalue_2 (`EnhancedInputSubsystemInterface.GetUserSettings` _returnvalue))
  ; Initialize player input
  ;; Add regular input mappings
  (`/Engine/EditorBlueprintResources/StandardMacros.IsValid` _returnvalue
    (:`Is Valid`
      (`EnhancedInputSubsystemInterface.AddMappingContext` _returnvalue "/Game/Input/IMC_Default.IMC_Default" 0 (struct))
      (if (not (`EnhancedInputUserSettings.IsMappingContextRegistered` _returnvalue_2 "/Game/Input/IMC_Default.IMC_Default"))
        (`EnhancedInputUserSettings.RegisterInputMappingContext` _returnvalue_2 "/Game/Input/IMC_Default.IMC_Default")))))

(event `EnhancedInput|/Game/Input/Actions/IA_Move`
  (params (ActionValue :type "Vector2D Structure") (ElapsedSeconds :type "Float (double-precision)") (TriggeredSeconds :type "Float (double-precision)") (InputAction :type "InputAction Object Reference" :default "/Game/Input/Actions/IA_Move.IA_Move"))
  (:`Triggered`
    (message `/Game/Blueprint/Players/BPI_Controls.CharacterMove` (`self.K2_GetPawn`) ActionValue_X ActionValue_Y)))

(event `EnhancedInput|/Game/Input/Actions/IA_MouseLook`
  (params (ActionValue :type "Vector2D Structure") (ElapsedSeconds :type "Float (double-precision)") (TriggeredSeconds :type "Float (double-precision)") (InputAction :type "InputAction Object Reference" :default "/Game/Input/Actions/IA_MouseLook.IA_MouseLook"))
  (:`Triggered`
    (bind _asgi_base (cast `/Game/Blueprint/GI_Base` (`GameplayStatics.GetGameInstance`)))
    (bind _savesettings (`/Game/Blueprint/GI_Base.SaveSettings` _asgi_base))
    (bind _returnvalue (`KismetMathLibrary.NormalizeToRange` (`/Game/Blueprint/Save/BP_SaveSettings.Sensitivity` _savesettings) 0.0 100.0))
    (message `/Game/Blueprint/Players/BPI_Controls.CharacterAim` (`self.K2_GetPawn`) (* (* _returnvalue ActionValue_X) (`KismetMathLibrary.SelectFloat` -1.0 1.0 (`/Game/Blueprint/Save/BP_SaveSettings.InvertXAxis` _savesettings))) (* (* _returnvalue ActionValue_Y) (`KismetMathLibrary.SelectFloat` -1.0 1.0 (`/Game/Blueprint/Save/BP_SaveSettings.InvertYAxis` _savesettings))))))

(event `self.ReceiveTick`
  (params (DeltaSeconds :type "Float (single-precision)"))
  (bind _interactpreview (`self.InteractPreview`))
  (bind _interactpreview_2 (`self.InteractPreview`))
  (if (and (`KismetSystemLibrary.IsValid` (`self.InteractPreview`)) (`KismetSystemLibrary.IsValid` (`self.HUD`)))
    (if (== (`self.GetViewTarget`) (`self.K2_GetPawn`))
      (bind (_outhit _returnvalue) (`self.AimFromPerspective`))
      (if _returnvalue
        (bind _returnvalue_2 (`self.GetComponentByClass` (`.HitActor` (`GameplayStatics.BreakHitResult` _outhit)) "/Game/Blueprint/BPC_Interactible.BPC_Interactible_C"))
        (`/Engine/EditorBlueprintResources/StandardMacros.IsValid` _returnvalue_2
          (:`Is Valid`
            (if (`/Game/Blueprint/BPC_Interactible.bInteractible` _returnvalue_2)
              (`|ExecutionSequence`
                (:`then_0`
                  (bind _output_get (set `/Game/Blueprint/Players/HUD/WB_InteractPreview.ref_Interactible` _returnvalue_2 _interactpreview))
                  (`|ExecutionSequence`
                    (:`then_0`
                      (if (not (`Widget.IsInViewport` _interactpreview_2))
                        (`UserWidget.AddToViewport` _interactpreview_2 0)))
                    (:`then_1`
                      (`/Game/Blueprint/Players/HUD/WB_InteractPreview.SetText` _interactpreview (`/Game/Blueprint/BPC_Interactible.InteractibleName` _output_get) (`/Game/Blueprint/BPC_Interactible.ActionDescription` _output_get)))))
                (:`then_1`
                  (`|ExecutionSequence`
                    (:`then_0`
                      (if (!= _returnvalue_2 (`self.Ref_lookedAtItem`))
                        (bind _ref_lookedatitem (`self.Ref_lookedAtItem` :!label _label)
                          (:`then`
                            (`/Game/Blueprint/BPC_Interactible.ToggleHighlight` _ref_lookedatitem false)
                            (`self.ReleaseInteract`)
                            (set `self.Ref_lookedAtItem` null))
                          (:`else`))))
                    (:`then_1`
                      (bind _output_get_2 (set `self.Ref_lookedAtItem` _returnvalue_2))
                      (`/Game/Blueprint/BPC_Interactible.ToggleHighlight` _output_get_2 true)))))
              (else
                (`Widget.RemoveFromParent` (`self.InteractPreview`) :!label _label_2)
                (goto _label))))
          (:`Is Not Valid`
            (goto _label_2)))
        (else
          (goto _label_2)))
      (else
        (goto _label_2)))))

(event `EnhancedInput|/Game/Input/Actions/IA_Jump`
  (params (ActionValue :type Boolean) (ElapsedSeconds :type "Float (double-precision)") (TriggeredSeconds :type "Float (double-precision)") (InputAction :type "InputAction Object Reference" :default "/Game/Input/Actions/IA_Jump.IA_Jump"))
  (:`Started`
    (message `/Game/Blueprint/Players/BPI_Controls.CharacterJump` (`self.K2_GetPawn`))))

(event `EnhancedInput|/Game/Input/Actions/IA_Interact`
  (params (ActionValue :type Boolean) (ElapsedSeconds :type "Float (double-precision)") (TriggeredSeconds :type "Float (double-precision)") (InputAction :type "InputAction Object Reference" :default "/Game/Input/Actions/IA_Interact.IA_Interact"))
  (:`Triggered`
    (bind (_outhit _returnvalue) (`self.AimFromPerspective`))
    (if _returnvalue
      (bind _returnvalue_2 (`self.GetComponentByClass` (`.HitActor` (`GameplayStatics.BreakHitResult` _outhit)) "/Game/Blueprint/BPC_Interactible.BPC_Interactible_C"))
      (`/Engine/EditorBlueprintResources/StandardMacros.IsValid` _returnvalue_2
        (:`Is Valid`
          (if (`/Game/Blueprint/BPC_Interactible.bInteractible` _returnvalue_2)
            (`self.ProgressInteract` _returnvalue_2)))
        (:`Is Not Valid`
          (`self.ReleaseInteract` :!label _label_3)))
      (else
        (goto _label_3))))
  (:`Canceled`
    (`self.ReleaseInteract` :!label _label_4))
  (:`Completed`
    (goto _label_4)))

(event `EnhancedInput|/Game/Input/Actions/IA_PrimaryFire`
  (params (ActionValue :type Boolean) (ElapsedSeconds :type "Float (double-precision)") (TriggeredSeconds :type "Float (double-precision)") (InputAction :type "InputAction Object Reference" :default "/Game/Input/Actions/IA_PrimaryFire.IA_PrimaryFire"))
  (bind _returnvalue (`self.K2_GetPawn`))
  (:`Started`
    (message `/Game/Blueprint/Players/BPI_Controls.HoldPrimary` _returnvalue))
  (:`Completed`
    (message `/Game/Blueprint/Players/BPI_Controls.ReleasePrimaryFire` _returnvalue)))

(event `EnhancedInput|/Game/Input/Actions/IA_Drop`
  (params (ActionValue :type Boolean) (ElapsedSeconds :type "Float (double-precision)") (TriggeredSeconds :type "Float (double-precision)") (InputAction :type "InputAction Object Reference" :default "/Game/Input/Actions/IA_Drop.IA_Drop"))
  (:`Triggered`
    (message `/Game/Blueprint/Players/BPI_Controls.DropItem` (`self.K2_GetPawn`))))

(event `ProgressInteract`
  (params (Target :type "/Game/Blueprint/BPC_Interactible Object Reference"))
  (bind _output_get (set `self.Progress` (+ (`self.Progress`) (`GameplayStatics.GetWorldDeltaSeconds`))))
  (if (>= _output_get (`/Game/Blueprint/BPC_Interactible.InteractDelay` Target))
    (`self.ReleaseInteract`)
    (message `/Game/Blueprint/Players/BPI_Controls.Interact` (`self.K2_GetPawn`) Target)))

(event `EnhancedInput|/Game/Input/Actions/IA_Menu`
  (params (ActionValue :type Boolean) (ElapsedSeconds :type "Float (double-precision)") (TriggeredSeconds :type "Float (double-precision)") (InputAction :type "InputAction Object Reference" :default "/Game/Input/Actions/IA_Menu.IA_Menu"))
  (:`Started`
    (bind _returnvalue (`|CreateWidget` "/Game/Widgets/Pause/WB_Menu.WB_Menu_C" self))
    (`UserWidget.AddToViewport` _returnvalue 0)))

(event `ReleaseInteract`
  (set `self.Progress` 0.0))

(event `/Game/Blueprint/Items/BPI_Items.Pick Up Item`
  (params (ref_item :type "/Game/Blueprint/Items/BP_Item Object Reference"))
  (message `/Game/Blueprint/Items/BPI_Items.Pick Up Item` (`self.K2_GetPawn`) ref_item))

(fn `AimFromPerspective`
  (returns (OutHit :type "HitResult Structure") (ReturnValue :type Boolean))
  (bind (_view_location _view_vector) (message `/Game/Blueprint/Players/BPI_Controls.GetViewLocation` (`self.K2_GetPawn`)))
  (bind (_outhit _returnvalue) (`KismetSystemLibrary.SphereTraceSingle` _view_location (+ _view_location (* _view_vector (`self.InteractionRange`))) 3.0 "TraceTypeQuery2"))
  (return _outhit _returnvalue))

(fn `UserConstructionScript`)