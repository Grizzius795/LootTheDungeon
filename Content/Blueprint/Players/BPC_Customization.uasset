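; Player component that applies and saves an adventurer's appearance: skin color, eyes, eyebrows, mouth and cheeks.
; On BeginPlay it creates a dynamic MI_Player material on the owner's mesh and applies customization from the owner's BP_AdventurerState.
; Each S_ event forwards to a setter that updates material parameters, then writes and saves the choice.
; Setters save to player state index 0, not the owner's, including during initial load.
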(event `self.ReceiveBeginPlay`
  (`self.S_InitAppearance`))

(event `S_InitAppearance`
  ; Init
  (`self.InitAppearance`)
  (`KismetSystemLibrary.PrintString` "Hello"))

(event `InitAppearance`
  ; Init
  (bind _asbp_adventurer (cast `/Game/Blueprint/Players/BP_Adventurer` (`self.GetOwner`)))
  (set `self.Mesh` (`Character.Mesh` _asbp_adventurer))
  (set `self.Player State` (`Pawn.PlayerState` _asbp_adventurer))
  (bind _returnvalue (`PrimitiveComponent.CreateDynamicMaterialInstance` (`self.Mesh`) 0 "/Game/Blueprint/Players/FBX/MI_Player.MI_Player" "None"))
  (set `self.DynamicPlayerMaterial` _returnvalue)
  (bind _asbp_adventurer_state (cast `/Game/Blueprint/Players/BP_AdventurerState` (`self.Player State`)))
  (bind _customcharacterdata (`/Game/Blueprint/Players/BP_AdventurerState.CustomCharacterData` _asbp_adventurer_state)
    (:`then`
      (bind (_skincolor _mouth _eyeshape _eyecolor _eyebrows _facedetails) (break `/Game/Blueprint/Mirror/Struct_CustomCharacter` (`/Game/Blueprint/Save/BP_SaveCharacter.Customization` _customcharacterdata)))
      (`self.S_SetSkinColor` _skincolor)
      (`self.S_SetMouth` _mouth)
      (`self.S_SetEyesShape` _eyeshape)
      (`self.S_SetEyeColor` _eyecolor)
      (`self.S_SetEyebrows` _eyebrows)
      (`self.S_SetCheeks` _facedetails))
    (:`else`)))

(event `S_SetMouth`
  (params (Mouth :type "/Game/Blueprint/Mirror/Struct_Mouth Structure"))
  ; Mouth
  (`self.SetMouth` Mouth))

(event `SetMouth`
  (params (Mouth :type "/Game/Blueprint/Mirror/Struct_Mouth Structure"))
  (bind _dynamicplayermaterial (`self.DynamicPlayerMaterial`))
  ; Mouth
  (`/Engine/EditorBlueprintResources/StandardMacros.IsValid` _dynamicplayermaterial
    (:`Is Valid`
      (`MaterialInstanceDynamic.SetTextureParameterValue` _dynamicplayermaterial "Mouth_Texture" (`.Texture_5_2768158047E989F3D1678B99347E5B3D` (break `/Game/Blueprint/Mirror/Struct_Mouth` Mouth)))
      (bind _asbp_adventurer_state (cast `/Game/Blueprint/Players/BP_AdventurerState` (`GameplayStatics.GetPlayerState` 0)))
      (bind _customcharacterdata (`/Game/Blueprint/Players/BP_AdventurerState.CustomCharacterData` _asbp_adventurer_state)
        (:`then`
          (setmembers `/Game/Blueprint/Mirror/Struct_CustomCharacter` :`StructRef` (`/Game/Blueprint/Save/BP_SaveCharacter.Customization` _customcharacterdata) :`Mouth` Mouth)
          (`/Game/Blueprint/Players/BP_AdventurerState.SaveCustomization` _asbp_adventurer_state))
        (:`else`)))))

(event `S_SetSkinColor`
  (params (Value :type "/Game/Blueprint/Mirror/Struct_SkinColors Structure"))
  ; SkinColor
  (`self.SetSkinColor` Value))

(event `SetSkinColor`
  (params (Value :type "/Game/Blueprint/Mirror/Struct_SkinColors Structure"))
  (bind _dynamicplayermaterial (`self.DynamicPlayerMaterial`))
  ; SkinColor
  (`/Engine/EditorBlueprintResources/StandardMacros.IsValid` _dynamicplayermaterial
    (:`Is Valid`
      (`MaterialInstanceDynamic.SetVectorParameterValue` _dynamicplayermaterial "SkinColor" (`.Color_9_89E0BCBA42CDB7980F13198DFAD18CFE` (break `/Game/Blueprint/Mirror/Struct_SkinColors` Value)))
      (bind _asbp_adventurer_state (cast `/Game/Blueprint/Players/BP_AdventurerState` (`GameplayStatics.GetPlayerState` 0)))
      (bind _customcharacterdata (`/Game/Blueprint/Players/BP_AdventurerState.CustomCharacterData` _asbp_adventurer_state)
        (:`then`
          (setmembers `/Game/Blueprint/Mirror/Struct_CustomCharacter` :`StructRef` (`/Game/Blueprint/Save/BP_SaveCharacter.Customization` _customcharacterdata) :`SkinColor` Value)
          (`/Game/Blueprint/Players/BP_AdventurerState.SaveCustomization` _asbp_adventurer_state))
        (:`else`)))))

(event `S_SetEyesShape`
  (params (Struct_Eyes :type "/Game/Blueprint/Mirror/Struct_Eyes Structure (by ref)"))
  ; EyeShape
  (`self.SetEyesShape` Struct_Eyes))

(event `SetEyesShape`
  (params (Struct_Eyes :type "/Game/Blueprint/Mirror/Struct_Eyes Structure (by ref)"))
  (bind ((`Shape_7_A2FC5ED64DA2B6DEB62774873B318201` _shape) (`Pupil_9_3BF1333B46FD0DC6BA1D69B98913D655` _pupil)) (break `/Game/Blueprint/Mirror/Struct_Eyes` Struct_Eyes))
  (bind _dynamicplayermaterial (`self.DynamicPlayerMaterial`))
  ; EyeShape
  (`/Engine/EditorBlueprintResources/StandardMacros.IsValid` _dynamicplayermaterial
    (:`Is Valid`
      (`MaterialInstanceDynamic.SetTextureParameterValue` _dynamicplayermaterial "Eyes_Contour_Texture" _shape)
      (`MaterialInstanceDynamic.SetTextureParameterValue` _dynamicplayermaterial "Eyes_Pupil_Texture" _pupil)
      (bind _asbp_adventurer_state (cast `/Game/Blueprint/Players/BP_AdventurerState` (`GameplayStatics.GetPlayerState` 0)))
      (bind _customcharacterdata (`/Game/Blueprint/Players/BP_AdventurerState.CustomCharacterData` _asbp_adventurer_state)
        (:`then`
          (setmembers `/Game/Blueprint/Mirror/Struct_CustomCharacter` :`StructRef` (`/Game/Blueprint/Save/BP_SaveCharacter.Customization` _customcharacterdata) :`EyeShape` Struct_Eyes)
          (`/Game/Blueprint/Players/BP_AdventurerState.SaveCustomization` _asbp_adventurer_state))
        (:`else`)))))

(event `S_SetEyeColor`
  (params (Struct_Eyes :type "/Game/Blueprint/Mirror/Struct_EyeColor Structure (by ref)"))
  ; EyeColor
  (`self.SetEyeColor` Struct_Eyes))

(event `SetEyeColor`
  (params (Struct_Eyes :type "/Game/Blueprint/Mirror/Struct_EyeColor Structure (by ref)"))
  (bind _dynamicplayermaterial (`self.DynamicPlayerMaterial`))
  ; EyeColor
  (`/Engine/EditorBlueprintResources/StandardMacros.IsValid` _dynamicplayermaterial
    (:`Is Valid`
      (`MaterialInstanceDynamic.SetVectorParameterValue` _dynamicplayermaterial "Pupil_Color" (`.Color_5_EAACF5744989DF194994CEA93556F639` (break `/Game/Blueprint/Mirror/Struct_EyeColor` Struct_Eyes)))
      (bind _asbp_adventurer_state (cast `/Game/Blueprint/Players/BP_AdventurerState` (`GameplayStatics.GetPlayerState` 0)))
      (bind _customcharacterdata (`/Game/Blueprint/Players/BP_AdventurerState.CustomCharacterData` _asbp_adventurer_state)
        (:`then`
          (setmembers `/Game/Blueprint/Mirror/Struct_CustomCharacter` :`StructRef` (`/Game/Blueprint/Save/BP_SaveCharacter.Customization` _customcharacterdata) :`EyeColor` Struct_Eyes)
          (`/Game/Blueprint/Players/BP_AdventurerState.SaveCustomization` _asbp_adventurer_state))
        (:`else`)))))

(event `S_SetEyebrows`
  (params (Struct_Eyebrows :type "/Game/Blueprint/Mirror/Struct_Eyebrows Structure (by ref)"))
  ; Eyebrows
  (`self.SetEyebrows` Struct_Eyebrows))

(event `SetEyebrows`
  (params (Struct_Eyebrows :type "/Game/Blueprint/Mirror/Struct_Eyebrows Structure (by ref)"))
  (bind _dynamicplayermaterial (`self.DynamicPlayerMaterial`))
  ; Eyebrows
  (`/Engine/EditorBlueprintResources/StandardMacros.IsValid` _dynamicplayermaterial
    (:`Is Valid`
      (`MaterialInstanceDynamic.SetTextureParameterValue` _dynamicplayermaterial "Brows_Texture" (`.Texture_7_FB7CA5CE4EF39D9A061F6693956FD8AB` (break `/Game/Blueprint/Mirror/Struct_Eyebrows` Struct_Eyebrows)))
      (bind _asbp_adventurer_state (cast `/Game/Blueprint/Players/BP_AdventurerState` (`GameplayStatics.GetPlayerState` 0)))
      (bind _customcharacterdata (`/Game/Blueprint/Players/BP_AdventurerState.CustomCharacterData` _asbp_adventurer_state)
        (:`then`
          (setmembers `/Game/Blueprint/Mirror/Struct_CustomCharacter` :`StructRef` (`/Game/Blueprint/Save/BP_SaveCharacter.Customization` _customcharacterdata) :`Eyebrows` Struct_Eyebrows)
          (`/Game/Blueprint/Players/BP_AdventurerState.SaveCustomization` _asbp_adventurer_state))
        (:`else`)))))

(event `S_SetCheeks`
  (params (Struct_Cheeks :type "/Game/Blueprint/Mirror/Struct_FaceDetails Structure (by ref)"))
  ; Cheeks
  (`self.SetCheeks` Struct_Cheeks))

(event `SetCheeks`
  (params (Struct_FaceDetails :type "/Game/Blueprint/Mirror/Struct_FaceDetails Structure (by ref)"))
  (bind _dynamicplayermaterial (`self.DynamicPlayerMaterial`))
  ; Cheeks
  (`/Engine/EditorBlueprintResources/StandardMacros.IsValid` _dynamicplayermaterial
    (:`Is Valid`
      (`MaterialInstanceDynamic.SetTextureParameterValue` _dynamicplayermaterial "Cheek_Texture" (`.Texture_7_FB7CA5CE4EF39D9A061F6693956FD8AB` (break `/Game/Blueprint/Mirror/Struct_FaceDetails` Struct_FaceDetails)))
      (bind _asbp_adventurer_state (cast `/Game/Blueprint/Players/BP_AdventurerState` (`GameplayStatics.GetPlayerState` 0)))
      (bind _customcharacterdata (`/Game/Blueprint/Players/BP_AdventurerState.CustomCharacterData` _asbp_adventurer_state)
        (:`then`
          (setmembers `/Game/Blueprint/Mirror/Struct_CustomCharacter` :`StructRef` (`/Game/Blueprint/Save/BP_SaveCharacter.Customization` _customcharacterdata) :`FaceDetails` Struct_FaceDetails)
          (`/Game/Blueprint/Players/BP_AdventurerState.SaveCustomization` _asbp_adventurer_state))
        (:`else`)))))