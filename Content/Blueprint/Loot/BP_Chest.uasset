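; BP_Chest is an interactible loot chest that spawns one randomly selected item when used, then turns off further interaction.
; On BeginPlay, SelectItem makes a weighted pick from the LootTable data table, using cumulative weights as map keys, and caches it as Content.
; Interacting spawns Content at the ItemSpawnPoint location.
; The construction script scales the chest mesh through a lookup of Size in ScaleBySize.
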(event `self.ReceiveBeginPlay`
  (bind _item (`self.SelectItem`))
  (set `self.Content` _item))

(event `self.BPC_Interactible.OnInteract`
  (params (Perpetrator :type "Actor Object Reference"))
  (set `/Game/Blueprint/BPC_Interactible.bInteractible` false (`self.BPC_Interactible`))
  (`|SpawnActorFromClass` (`self.Content`) (`KismetMathLibrary.MakeTransform` (`SceneComponent.K2_GetComponentLocation` (`self.ItemSpawnPoint`))) "Undefined" "MultiplyWithRoot" null null))

(fn `SelectItem`
  (returns (Item :type "/Game/Blueprint/Items/BP_Item Class Reference"))
  (locals (LootTableWeight :type "Map of Float (double-precision) to /Game/Blueprint/Items/BP_Item Class Reference") (Max :type "Float (double-precision)") (RandomPick :type "Float (double-precision)" :default 0.0) (FoundItem :type "/Game/Blueprint/Items/BP_Item Class Reference"))
  (bind _outrownames (`DataTableFunctionLibrary.GetDataTableRowNames` (`self.LootTable`)))
  (for _array_element _outrownames
    (bind _returnvalue (`|GetDataTableRow` (`self.LootTable`) _array_element)
      (:`then`
        (bind (_item _weight) (break `/Game/Blueprint/Loot/Struct_LootTableEntry` _returnvalue))
        (bind _returnvalue_2 (+ (`local.Max`) _weight))
        (`BlueprintMapLibrary.Map_Add` (`local.LootTableWeight`) _returnvalue_2 _item)
        (set `local.Max` _returnvalue_2))))
  (set `local.RandomPick` (`KismetMathLibrary.RandomFloatInRange` 0.0 (`local.Max`)))
  (bind (_keypin _valuepin) (`|MapForEach` (`local.LootTableWeight`))
    (:`then`
      (if (> _keypin (`local.RandomPick`))
        (bind _output_get (set `local.FoundItem` _valuepin))
        (return _output_get)))))

(fn `UserConstructionScript`
  (`SceneComponent.SetWorldScale3D` (`self.ChestAnimations_V001_nnca`) (`KismetMathLibrary.Conv_DoubleToVector` (`BlueprintMapLibrary.Map_Find` (`self.ScaleBySize`) (`self.Size`)))))