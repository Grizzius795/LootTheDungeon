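; Dungeon exit door that opens once when interacted with, provided it has been allowed to open.
; Its interactible component's OnInteract checks the CanOpen flag, then plays the door's actor sequence through a DoOnce.
; SetCanOpen lets outside logic unlock it, and SetQuest forwards a quest to the door's WB_DoorQuestDisplay widget.
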(event `self.BPC_Interactible.OnInteract`
  (params (Perpetrator :type "Actor Object Reference"))
  (if (`self.bCanOpen`)
    (`/Engine/EditorBlueprintResources/StandardMacros.DoOnce` false
      (:`Completed`
        (`ActorSequenceComponent.PlaySequence` (`self.ActorSequence`))))))

(fn `SetCanOpen`
  (params (bCanOpen :type Boolean))
  (set `self.bCanOpen` bCanOpen))

(fn `SetQuest`
  (params (Quest :type "/Game/Blueprint/Quests/BP_Quest Object Reference"))
  (bind _aswb_door_quest_display (cast `/Game/Blueprint/Quests/WB_DoorQuestDisplay` (`WidgetComponent.GetWidget` (`self.Widget`))))
  (`/Game/Blueprint/Quests/WB_DoorQuestDisplay.SetQuest` _aswb_door_quest_display Quest))

(fn `UserConstructionScript`)