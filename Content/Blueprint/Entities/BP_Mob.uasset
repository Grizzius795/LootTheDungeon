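; BP_Mob is a mob entity that handles its own unconscious and death reactions through health component events.
; Going unconscious puts the physical animation component into ragdoll a tick later.
; Death, guarded to run once, swaps the mesh's first material for a dynamic dissolve instance and animates it by timeline before destroying the actor.
; A delayed Niagara explosion spawns at the hips socket during the dissolve.
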(event `self.ReceiveBeginPlay`)

(event `self.BPC_Health.OnUnconscious`
  (`KismetSystemLibrary.DelayUntilNextTick`)
  (`/Game/Blueprint/BPC_PhysicalAnim.EnterRagdoll` (`self.BPC_PhysicalAnim`)))

(event `DissolveBody`
  (`|ExecutionSequence`
    (:`then_0`
      (bind _returnvalue (`KismetMaterialLibrary.CreateDynamicMaterialInstance` "/Game/Materials/M_Dissolve.M_Dissolve"))
      (bind _output_get (set `self.DissolveMaterial` _returnvalue))
      (`PrimitiveComponent.SetMaterial` (`self.Mesh`) 0 _output_get))
    (:`then_1`
      (bind (_direction _dissolve) (`Timeline|Timeline` :!via `PlayFromStart`)
        (:`Update`
          (`MaterialInstanceDynamic.SetScalarParameterValue` (`self.DissolveMaterial`) "Dissolve" _dissolve))
        (:`Finished`
          (`self.K2_DestroyActor`))))
    (:`then_2`
      (`KismetSystemLibrary.Delay` 1.2)
      (`NiagaraFunctionLibrary.SpawnSystemAtLocation` "/Game/Blueprint/Entities/NG_DeathExplosion.NG_DeathExplosion" (`SceneComponent.GetSocketLocation` (`self.Mesh`) "Hips")))))

(event `self.BPC_Health.OnDeath`
  (`/Engine/EditorBlueprintResources/StandardMacros.DoOnce` false
    (:`Completed`
      (`KismetSystemLibrary.DelayUntilNextTick`)
      (`self.DissolveBody`))))

(fn `UserConstructionScript`)