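; BP_Cult is an actor that keeps track of cultists organized into groups, each with a member list and a leader.
; CreateGroup promotes its first member, makes them the leader of a new group struct and returns that group's index.
; AddCultistToGroup adds unique members by group index, while CultistInGroup searches all groups and returns whether a cultist belongs and to which index.
; The event graph and construction script hold no logic.
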(fn `AddCultistToGroup`
  (params (GroupID :type Integer) (Cultist :type "/Game/Blueprint/Entities/Cultist/Mob_Cultist Object Reference"))
  (`KismetArrayLibrary.Array_AddUnique` (`.Members_5_5A0C514E456D19BC49694FB508F7C5C2` (break `/Game/Blueprint/Entities/Cultist/Struct_CultistGroup` (`|GetArrayItem` (`self.Groups`) GroupID))) (`local.Cultist`)))

(fn `CreateGroup`
  (params (`First Member` :type "/Game/Blueprint/Entities/Cultist/Mob_Cultist Object Reference"))
  (returns (NewGroupID :type Integer))
  (`/Game/Blueprint/Entities/Cultist/Mob_Cultist.Promote` `First Member`)
  (bind _returnvalue (`KismetArrayLibrary.Array_Add` (`self.Groups`) (make `/Game/Blueprint/Entities/Cultist/Struct_CultistGroup` (`|MakeArray` `First Member`) `First Member`)))
  (return _returnvalue))

(fn `CultistInGroup`
  (params (Cultist :type "/Game/Blueprint/Entities/Cultist/Mob_Cultist Object Reference"))
  (returns (Out :type Boolean) (`Group ID` :type Integer))
  (for (_array_element _array_index) (`self.Groups`)
    (if (`KismetArrayLibrary.Array_Contains` (`.Members_5_5A0C514E456D19BC49694FB508F7C5C2` (break `/Game/Blueprint/Entities/Cultist/Struct_CultistGroup` _array_element)) (`local.Cultist`))
      (return true _array_index)))
  (return false 0))

(fn `UserConstructionScript`)