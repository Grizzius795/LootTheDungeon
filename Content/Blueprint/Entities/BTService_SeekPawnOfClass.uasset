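; Behavior tree service that records a pawn of a chosen class in the blackboard when the controlled AI pawn sees it.
; On activation it binds to the OnSeePawn event of the controlled pawn's PawnSensingComponent.
; Each sighting whose class exactly matches PawnClassToSeek is written to the SeenPawn key, along with a debug print.
; The file shows no unbinding or clearing of the key.
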(event `self.ReceiveActivationAI`
  (params (OwnerController :type "AIController Object Reference") (ControlledPawn :type "Pawn Object Reference"))
  (add `PawnSensingComponent.OnSeePawn` (`Actor.GetComponentByClass` ControlledPawn "/Script/AIModule.PawnSensingComponent") (`|CreateDelegate` :!event `BTService_SeekPawnOfClass_AutoGenFunc`)))

(fn `BTService_SeekPawnOfClass_AutoGenFunc`
  (params (Pawn :type "Pawn Object Reference"))
  (if (== (`GameplayStatics.GetObjectClass` Pawn) (`self.PawnClassToSeek`))
    (`BTFunctionLibrary.SetBlackboardValueAsObject` (`self.SeenPawn`) (`local.Pawn`))
    (`KismetSystemLibrary.PrintString` "Found player !")))