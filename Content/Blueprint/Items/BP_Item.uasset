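; BP_Item is a data-driven world item that characters can pick up, hold and drop, with an empty PrimaryUse event.
; GetItemData supplies the mesh at construction and the interaction name at BeginPlay.
; Interacting sends a pickup message to the perpetrator and disables further interaction, which nothing here re-enables.
; Attaching disables physics and collision, snaps to the parent and records the holder; detaching restores physics and collision and clears it.
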(event `self.ReceiveBeginPlay`
  (set `/Game/Blueprint/BPC_Interactible.InteractibleName` (`.Name_3_9EB4971C40F19E6137E72A90E671852B` (break `/Game/Blueprint/Items/Struct_Item` (`/Game/Blueprint/Items/BPFL_Items.GetItemData` (`self.Item`)))) (`self.BPC_Interactible`)))

(event `PrimaryUse`)

(event `self.BPC_Interactible.OnInteract`
  (params (Perpetrator :type "Actor Object Reference"))
  (message `/Game/Blueprint/Items/BPI_Items.Pick Up Item` Perpetrator self)
  (set `/Game/Blueprint/BPC_Interactible.bInteractible` false (`self.BPC_Interactible`)))

(fn `AttachToComponent`
  (params (Parent :type "SceneComponent Object Reference"))
  (`PrimitiveComponent.SetSimulatePhysics` (`self.StaticMesh`) false)
  (`PrimitiveComponent.SetCollisionEnabled` (`self.StaticMesh`) "NoCollision")
  (`self.K2_AttachToComponent` Parent "None" "SnapToTarget" "SnapToTarget" "KeepRelative" false)
  (set `self.ref_Holder` (`ActorComponent.GetOwner` (`local.Parent`))))

(fn `DetachFromParent`
  (`self.K2_DetachFromActor` "KeepWorld" "KeepWorld" "KeepWorld")
  (`PrimitiveComponent.SetSimulatePhysics` (`self.StaticMesh`) true)
  (`PrimitiveComponent.SetCollisionEnabled` (`self.StaticMesh`) "QueryAndPhysics")
  (set `self.ref_Holder` null))

(fn `SetItem`
  (params (ItemName :type Name))
  (bind (_out_data _is_valid) (`/Game/Blueprint/Items/BPFL_Items.GetItemData` ItemName))
  (bind _staticmesh (`self.StaticMesh`))
  (if _is_valid
    (`StaticMeshComponent.SetStaticMesh` _staticmesh (`.Mesh_8_30BF231249DF68B153E86D982AE2D2B3` (break `/Game/Blueprint/Items/Struct_Item` _out_data)))
    (else
      (`StaticMeshComponent.SetStaticMesh` _staticmesh null))))

(fn `UserConstructionScript`
  (`self.SetItem` (`self.Item`)))