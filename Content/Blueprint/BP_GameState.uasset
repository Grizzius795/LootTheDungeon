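; Game state Blueprint that runs the tavern-to-dungeon flow, from loading screen to game over.
; StartDungeon triggers BP_DungeonGenerator, binds its completion event, starts an exploration timer and binds player death events; the Tavern level is unloaded as loading ends.
; A game-over widget appears once all players are dead, guarded by a DoOnce reset each run.
; It also retries until player state exists to play tavern music, applies customized appearances, relays joins and shows biome cards.
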(event `self.ReceiveBeginPlay`
  (bind _returnvalue (`GameplayStatics.GetPlayerState` 0))
  (`/Engine/EditorBlueprintResources/StandardMacros.IsValid` _returnvalue :!label _label
    (:`Is Valid`
      (bind _asbp_adventurer_state (cast `/Game/Blueprint/Players/BP_AdventurerState` _returnvalue))
      (`/Game/Blueprint/Players/BP_AdventurerState.PlayBGM` _asbp_adventurer_state "/Game/Audio/BGM/BGM_Tavern.BGM_Tavern"))
    (:`Is Not Valid`
      (`KismetSystemLibrary.Delay` 0.2)
      (goto _label))))

(event `StartloadingScreen`
  (bind _returnvalue (`|CreateWidget` "/Game/Widgets/LoadingScreen/WB_Loading.WB_Loading_C"))
  (bind _output_get (set `self.LoadingScreen` _returnvalue))
  (`UserWidget.AddToViewport` _output_get 0))

(event `ApplyPlayerAppearances`
  (for _index (range (`GameplayStatics.GetNumPlayerStates`))
    (bind _returnvalue (`self.GetComponentByClass` (`PlayerState.GetPawn` (`GameplayStatics.GetPlayerState` _index)) "/Game/Blueprint/Players/BPC_Customization.BPC_Customization_C"))
    (`/Engine/EditorBlueprintResources/StandardMacros.IsValid` _returnvalue
      (:`Is Valid`
        (`/Game/Blueprint/Players/BPC_Customization.S_InitAppearance` _returnvalue)))))

(event `EndLoadingScreen`
  (`/Game/Widgets/LoadingScreen/WB_Loading.FinishLoading` (`self.LoadingScreen`)))

(event `PlayerLogin`
  (params (`New player` :type "PlayerController Object Reference"))
  (`self.OnPlayerJoin` `New player`))

(event `ShowBiomeCard`
  (bind _returnvalue (`|CreateWidget` "/Game/Widgets/BiomeCard/WB_BiomeCard.WB_BiomeCard_C"))
  (`UserWidget.AddToViewport` _returnvalue 0))

(event `CountPlayers`
  (bind _outactors (`GameplayStatics.GetAllActorsOfClass` "/Game/Blueprint/Players/BP_AdventurerController.BP_AdventurerController_C"))
  (bind _output_get (set `self.Players` _outactors))
  (for _array_element _output_get
    (add `/Game/Blueprint/Damage/BPC_Health.OnDeath` (`self.GetComponentByClass` (`Controller.K2_GetPawn` _array_element) "/Game/Blueprint/Damage/BPC_Health.BPC_Health_C") (`|CreateDelegate` :!event `OnPlayerDeath`))))

(event `StartDungeon`
  (`self.StartLoadingScreen`)
  (bind _returnvalue (`GameplayStatics.GetActorOfClass` "/Game/Maps/Dungeon/BP_DungeonGenerator.BP_DungeonGenerator_C"))
  (`/Engine/EditorBlueprintResources/StandardMacros.IsValid` _returnvalue
    (:`Is Valid`
      (`DungeonGeneratorBase.Generate` _returnvalue)
      (add `/Game/Maps/Dungeon/BP_DungeonGenerator.FinishedGeneration` _returnvalue (`|CreateDelegate` :!event `CustomEvent`))
      (set `self.ExplorationTime` 0)
      (`KismetSystemLibrary.K2_SetTimerDelegate` (`|CreateDelegate` :!event `IncrementTimer`) 1.0 true)
      (`self.CountPlayers`)
      (`self.ResetGameOverDisplay`))
    (:`Is Not Valid`
      (`KismetSystemLibrary.PrintString` "Failed to get Dungeon Generator"))))

(event `CustomEvent`
  (`GameplayStatics.UnloadStreamLevelBySoftObjectPtr` "/Game/Maps/Tavern/Tavern.Tavern")
  (`self.EndLoadingScreen`))

(event `OnPlayerDeath`
  (if (`self.CheckAreAllPlayersDead`)
    (`self.DisplayGameOverScreen`)))

(event `DisplayGameOverScreen`
  (`/Engine/EditorBlueprintResources/StandardMacros.DoOnce` false :!label _label_2
    (:`Completed`
      (bind _returnvalue (`|CreateWidget` "/Game/Widgets/GameOverScreen/WB_GameOver.WB_GameOver_C"))
      (`UserWidget.AddToViewport` _returnvalue 0))))

(event `ResetGameOverDisplay`
  (goto _label_2 :!via `Reset`))

(fn `CheckAreAllPlayersDead`
  (returns (bAllDead :type Boolean))
  (locals (bNotAllDead :type Boolean))
  (for _array_element (`self.Players`)
    (if (not (`/Game/Blueprint/Players/BP_AdventurerController.bIsDead` _array_element))
      (set `local.bNotAllDead` true)))
  (return (not (`local.bNotAllDead`))))

(fn `IncrementTimer`
  (`/Engine/EditorBlueprintResources/StandardMacros.IncrementInt` (`self.ExplorationTime`)))

(fn `UserConstructionScript`)