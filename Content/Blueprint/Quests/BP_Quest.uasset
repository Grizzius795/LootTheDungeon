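; BP_Quest is a quest Blueprint that tracks progress toward completion and gates the dungeon's end door.
; SetupDoor finds the BP_DungeonEndDoor in the world and registers the quest with it.
; UpdateProgress stores new progress, broadcasts OnUpdateProgress, and calls SucceedQuest at the final value, which marks the quest finished and lets the door open.
; SetupQuest takes a dungeon but only returns true here.
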(fn `SetupDoor`
  (bind _returnvalue (`GameplayStatics.GetActorOfClass` "/Game/Blueprint/BP_DungeonEndDoor.BP_DungeonEndDoor_C"))
  (`/Game/Blueprint/BP_DungeonEndDoor.SetQuest` _returnvalue self))

(fn `SetupQuest`
  (params (Dungeon :type "DungeonGraph Object Reference"))
  (returns (success :type Boolean))
  (return true))

(fn `SucceedQuest`
  (set `self.bIsFinished` true)
  (bind _returnvalue (`GameplayStatics.GetActorOfClass` "/Game/Blueprint/BP_DungeonEndDoor.BP_DungeonEndDoor_C"))
  (`/Game/Blueprint/BP_DungeonEndDoor.SetCanOpen` _returnvalue true))

(fn `UpdateProgress`
  (params (NewProgress :type Integer))
  (set `self.CurrentProgress` NewProgress)
  (`self.OnUpdateProgress`)
  (if (>= (`self.CurrentProgress`) (`self.FinalProgress`))
    (`self.SucceedQuest`)))

(fn `UserConstructionScript`)