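; Dungeon quest that gates a mechanical door behind levers placed at random spawn points.
; Setup makes up to 50 random picks among BP_SpawnPoint actors, spawning and binding a lever at unused ones until FinalProgress is met, then calls SetupDoor or reports failure.
; The toggle handler recounts activated levers and passes the total to UpdateProgress.
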(fn `Quest_MecanicalDoor_AutoGenFunc`
  (params (NewValue :type Boolean))
  (locals (L_progress :type Integer))
  (for _array_element (`self.Levers`)
    (if (`/Game/Blueprint/BP_Lever.bActivated` _array_element)
      (`/Engine/EditorBlueprintResources/StandardMacros.IncrementInt` (`local.L_progress`))))
  (`self.UpdateProgress` (`local.L_progress`)))

(fn `SetupQuest`
  (params (Dungeon :type "DungeonGraph Object Reference"))
  (returns (success :type Boolean))
  (locals (SpawnPoint :type "/Game/Blueprint/BP_SpawnPoint Object Reference"))
  (bind _levers (`self.Levers`))
  (for _ (range 51)
    (bind _outactors (`GameplayStatics.GetAllActorsOfClass` "/Game/Blueprint/BP_SpawnPoint.BP_SpawnPoint_C"))
    (bind _outitem (`KismetArrayLibrary.Array_Random` _outactors))
    (`/Engine/EditorBlueprintResources/StandardMacros.IsValid` _outitem
      (:`Is Valid`
        (bind _output_get (set `local.SpawnPoint` _outitem))
        (if (not (`/Game/Blueprint/BP_SpawnPoint.bUsed` _output_get))
          (bind _out (`/Game/Blueprint/BP_SpawnPoint.SpawnActor` (`local.SpawnPoint`) "/Game/Blueprint/BP_Lever.BP_Lever_C"))
          (bind _asbp_lever (cast `/Game/Blueprint/BP_Lever` _out))
          (`KismetArrayLibrary.Array_Add` _levers _asbp_lever)
          (add `/Game/Blueprint/BP_Lever.OnToggle` _asbp_lever (`|CreateDelegate` :!event `Quest_MecanicalDoor_AutoGenFunc`))
          (if (>= (`KismetArrayLibrary.Array_Length` _levers) (`self.FinalProgress`))
            (break))))))
  (if (>= (`KismetArrayLibrary.Array_Length` (`self.Levers`)) (`self.FinalProgress`))
    (`self.SetupDoor`)
    (return true)
    (else
      (return false))))

(fn `UserConstructionScript`
  (`parent.UserConstructionScript`))