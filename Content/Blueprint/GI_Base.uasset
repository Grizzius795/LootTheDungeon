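; Base Game Instance that owns persistent player settings and multiplayer session flow.
; Init loads or creates the BP_SaveSettings save; setters store mic gain and volumes immediately, but only mic gain is applied here, via console command.
; Hosting (Advanced Sessions, listen server on L_Main), accepting invites and returning to the main menu each destroy any existing session first, proceeding even if that fails.
; LoadSettings only casts the save object.
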(event `self.ReceiveInit`
  (`|ExecutionSequence`
    (:`then_0`
      (bind _returnvalue (`GameplayStatics.DoesSaveGameExist` "Settings"))
      (if _returnvalue
        (bind _returnvalue_2 (`GameplayStatics.LoadGameFromSlot` "Settings"))
        (bind _asbp_save_settings (cast `/Game/Blueprint/Save/BP_SaveSettings` _returnvalue_2))
        (set `self.SaveSettings` _asbp_save_settings)
        (else
          (bind _returnvalue_3 (`GameplayStatics.CreateSaveGameObject` "/Game/Blueprint/Save/BP_SaveSettings.BP_SaveSettings_C"))
          (bind _output_get (set `self.SaveSettings` _returnvalue_3))
          (`GameplayStatics.SaveGameToSlot` _output_get "Settings"))))))

(event `CreateSession`
  (params (`Session Name` :type String) (`Max Players` :type Integer) (bIsPublic :type Boolean))
  (`DestroySessionCallbackProxy.DestroySession` (`GameplayStatics.GetPlayerController` 0)
    (:`OnSuccess`
      _)
    (:`OnFailure`
      _))
  (`CreateSessionCallbackProxyAdvanced.CreateAdvancedSession` (`|MakeArray` (`AdvancedSessionsLibrary.MakeLiteralSessionPropertyString` "SessionName" `Session Name`)) (`GameplayStatics.GetPlayerController` 0) `Max Players` 0 false true false true true false false false bIsPublic
    (:`OnSuccess`
      (`GameplayStatics.OpenLevelBySoftObjectPtr` "/Game/L_Main.L_Main" true "listen"))))

(event `self.OnSessionInviteAccepted`
  (params (LocalPlayerNum :type Integer) (PersonInvited :type "BPUniqueNetId Structure") (SessionToJoin :type "BlueprintSessionResult Structure (by ref)"))
  (`DestroySessionCallbackProxy.DestroySession` (`GameplayStatics.GetPlayerController` 0)
    (:`OnSuccess`
      _)
    (:`OnFailure`
      _))
  (`JoinSessionCallbackProxy.JoinSession` (`GameplayStatics.GetPlayerController` 0) SessionToJoin
    (:`OnSuccess`
      (`KismetSystemLibrary.PrintString` "successfully joined session"))
    (:`OnFailure`
      (`KismetSystemLibrary.PrintString` "Failed to join session"))))

(event `ReturnToMainMenu`
  (`DestroySessionCallbackProxy.DestroySession` (`GameplayStatics.GetPlayerController` 0)
    (:`OnSuccess`
      _)
    (:`OnFailure`
      _))
  (`GameplayStatics.OpenLevelBySoftObjectPtr` "/Game/Widgets/MainMenu/L_MainMenu.L_MainMenu"))

(fn `LoadSettings`
  (cast `/Game/Blueprint/Save/BP_SaveSettings` (`self.SaveSettings`)))

(fn `SetMasterVolume`
  (params (MasterVolume :type Integer))
  (bind _savesettings (`self.SaveSettings`))
  (set `/Game/Blueprint/Save/BP_SaveSettings.MasterVolume` MasterVolume _savesettings)
  (`GameplayStatics.SaveGameToSlot` _savesettings "settings"))

(fn `SetMicGain`
  (params (Param :type Name))
  (bind _savesettings (`self.SaveSettings`))
  (`|ExecutionSequence`
    (:`then_0`
      (switch `name` Param
        (:`Low`
          (`KismetSystemLibrary.ExecuteConsoleCommand` "voice.MicInputGain 0.5" null))
        (:`Medium`
          (`KismetSystemLibrary.ExecuteConsoleCommand` "voice.MicInputGain 1" null))
        (:`High`
          (`KismetSystemLibrary.ExecuteConsoleCommand` "voice.MicInputGain 2" null))))
    (:`then_1`
      (set `/Game/Blueprint/Save/BP_SaveSettings.MicGain` (`local.Param`) _savesettings)
      (`GameplayStatics.SaveGameToSlot` _savesettings "settings"))))

(fn `SetMusicVolume`
  (params (MusicVolume :type Integer))
  (bind _savesettings (`self.SaveSettings`))
  (set `/Game/Blueprint/Save/BP_SaveSettings.MusicVolume` MusicVolume _savesettings)
  (`GameplayStatics.SaveGameToSlot` _savesettings "settings"))

(fn `SetSFXVolume`
  (params (SFXVolume :type Integer))
  (bind _savesettings (`self.SaveSettings`))
  (set `/Game/Blueprint/Save/BP_SaveSettings.SFXVolume` SFXVolume _savesettings)
  (`GameplayStatics.SaveGameToSlot` _savesettings "settings"))