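; Actor component that drives physical animation, hit reactions and ragdoll on the owning character's skeletal mesh.
; It creates a PhysicalAnimationComponent at BeginPlay and simulates bodies below the upper-body root.
; Hits apply a profile and bone impulse, then Tick eases physics blend weight out.
; During ragdoll, the actor follows the root bone; CheckRagdollCanStop signals when a living body is grounded and either still or timed out.
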(event `self.ReceiveBeginPlay`
  (bind _upperbodyroot (`self.UpperBodyRoot`))
  (bind _returnvalue (`|AddComponentByClass` (`self.GetOwner`) "/Script/Engine.PhysicalAnimationComponent"))
  (set `self.Ref_PhysicalAnimationComponent` _returnvalue)
  (bind _output_get (set `self.ref_mesh` (`Actor.GetComponentByClass` (`self.GetOwner`) "/Script/Engine.SkeletalMeshComponent")))
  (`PhysicalAnimationComponent.SetSkeletalMeshComponent` (`self.Ref_PhysicalAnimationComponent`) _output_get)
  (`PhysicalAnimationComponent.ApplyPhysicalAnimationSettingsBelow` (`self.Ref_PhysicalAnimationComponent`) _upperbodyroot (`self.DefaultPhysicalAnimData`) true)
  (`SkeletalMeshComponent.SetAllBodiesBelowSimulatePhysics` (`self.ref_mesh`) _upperbodyroot true false))

(event `TogglePhysicalAnimation`
  (`SkeletalMeshComponent.SetAllBodiesBelowSimulatePhysics` (`self.ref_mesh`) "Hips" true false)
  (`SkeletalMeshComponent.SetAllBodiesBelowPhysicsBlendWeight` (`self.ref_mesh`) "Hips" 0.5 false true))

(event `HitReaction`
  (params (HitInfo :type "/Game/Blueprint/Items/Struct_hitInfo Structure"))
  (bind (_hitbonename _hitlocation _hitnormal _hitdirection) (break `/Game/Blueprint/Items/Struct_hitInfo` HitInfo))
  (set `self.HitReactionTimeRemaining` (+ (`self.HitReactionTimeRemaining`) 2.0))
  (`SkeletalMeshComponent.SetAllBodiesBelowSimulatePhysics` (`self.ref_mesh`) "Hips" true false)
  (`PhysicalAnimationComponent.ApplyPhysicalAnimationProfileBelow` (`self.Ref_PhysicalAnimationComponent`) "Hips" "HitReaction" false false)
  (`PrimitiveComponent.AddImpulse` (`self.ref_mesh`) (* _hitdirection 5000.0) (`KismetMathLibrary.SelectName` "Spine" _hitbonename (== _hitbonename "Hips")) true)
  (`KismetSystemLibrary.Delay` 0.2)
  (`self.SetComponentTickEnabled` true))

(event `S_HitReactionRecovery`
  (`self.HitReactionRecovery`))

(event `HitReactionRecovery`
  (bind _ref_mesh (`self.ref_mesh`))
  (bind _output_get (set `self.HitReactionTimeRemaining` (`KismetMathLibrary.FInterpTo` (`self.HitReactionTimeRemaining`) 0.0 (`GameplayStatics.GetWorldDeltaSeconds`) 10.0)))
  (if (<= _output_get 0.0)
    (set `self.HitReactionTimeRemaining` 0.0)
    (if (not (`SceneComponent.IsSimulatingPhysics` _ref_mesh "None"))
      (`SkeletalMeshComponent.SetAllBodiesBelowSimulatePhysics` _ref_mesh "Hips" false true)
      (`self.SetComponentTickEnabled` false))
    (else
      (`SkeletalMeshComponent.SetAllBodiesBelowPhysicsBlendWeight` (`self.ref_mesh`) "Hips" (`KismetMathLibrary.FMin` (`self.HitReactionTimeRemaining`) 1.0) false true))))

(event `self.ReceiveTick`
  (params (DeltaSeconds :type "Float (single-precision)"))
  (if (`self.bInRagdoll`)
    (`self.GetRootTransform`)
    (else
      (`self.HitReactionRecovery`))))

(event `S_ToggleSimulateRagdollPhysics`
  (params (bSimulate :type Boolean))
  (`PrimitiveComponent.SetSimulatePhysics` (`self.ref_mesh`) bSimulate)
  (`self.SetComponentTickEnabled` bSimulate))

(event `GetRootTransform`
  (bind _output_get (set `self.RootTransform` (`SkinnedMeshComponent.GetBoneTransform` (`self.ref_mesh`) (`self.RootBoneName`) "RTS_World")))
  (`Actor.K2_SetActorLocation` (`self.GetOwner`) (.location _output_get) false false))

(event `CheckRagdollCanStop`
  (bind _ref_mesh (`self.ref_mesh`))
  (bind _returnvalue (`SceneComponent.GetSocketLocation` _ref_mesh "hips"))
  (bind _returnvalue_2 (`Actor.GetComponentByClass` (`self.GetOwner`) "/Game/Blueprint/Damage/BPC_Health.BPC_Health_C"))
  (`/Engine/EditorBlueprintResources/StandardMacros.IsValid` _returnvalue_2
    (:`Is Valid`
      (if (> (`/Game/Blueprint/Damage/BPC_Health.HP` _returnvalue_2) 0)
        (bind (_outhit _returnvalue_3) (`KismetSystemLibrary.LineTraceSingle` :`Start` _returnvalue :`End` (+ _returnvalue (* (`KismetMathLibrary.Vector_Up`) -50.0)) :`TraceChannel` "TraceTypeQuery1" :`DrawDebugType` "ForDuration" :!label _label))
        (if (and _returnvalue_3 (or (< (`KismetMathLibrary.VSize` (`SceneComponent.GetComponentVelocity` _ref_mesh)) 1.0) (`self.bMustEndRagdoll`)))
          (set `self.bMustEndRagdoll` false)
          (`self.OnRagdollStopMoving`)
          (`KismetSystemLibrary.K2_ClearAndInvalidateTimerHandle` (`self.RagdollCheckHandle`)))))
    (:`Is Not Valid`
      (goto _label))))

(event `CustomEvent`
  (set `self.bMustEndRagdoll` true))

(fn `EndRagdoll`
  (bind _ref_mesh (`self.ref_mesh`))
  (bind _upperbodyroot (`self.UpperBodyRoot`))
  (set `self.bInRagdoll` false)
  (`PhysicalAnimationComponent.ApplyPhysicalAnimationProfileBelow` (`self.Ref_PhysicalAnimationComponent`) (`self.RootBoneName`) "None" true false)
  (`PhysicalAnimationComponent.ApplyPhysicalAnimationSettingsBelow` (`self.Ref_PhysicalAnimationComponent`) _upperbodyroot (`self.DefaultPhysicalAnimData`) true)
  (`SkeletalMeshComponent.SetAllBodiesBelowSimulatePhysics` _ref_mesh (`self.RootBoneName`) false true)
  (`SkeletalMeshComponent.SetAllBodiesBelowSimulatePhysics` _ref_mesh _upperbodyroot true false)
  (`CharacterMovementComponent.SetMovementMode` (`Actor.GetComponentByClass` (`self.GetOwner`) "/Script/Engine.CharacterMovementComponent") "MOVE_Walking" 0)
  (`SceneComponent.K2_SetRelativeLocationAndRotation` (`self.ref_mesh`) (0.0 0.0 -88.0) (struct :`Yaw` -90.0) false false))

(fn `EnterRagdoll`
  (bind _ref_mesh (`self.ref_mesh`))
  (`PhysicalAnimationComponent.ApplyPhysicalAnimationProfileBelow` (`self.Ref_PhysicalAnimationComponent`) (`self.RootBoneName`) "Ragdoll" true false)
  (`SkeletalMeshComponent.SetAllBodiesBelowSimulatePhysics` _ref_mesh (`self.RootBoneName`) true false)
  (`PrimitiveComponent.SetCollisionObjectType` _ref_mesh "ECC_PhysicsBody")
  (`CharacterMovementComponent.SetMovementMode` (`Actor.GetComponentByClass` (`self.GetOwner`) "/Script/Engine.CharacterMovementComponent") "MOVE_None" 0)
  (`self.S_ToggleSimulateRagdollPhysics` true)
  (set `self.bInRagdoll` true)
  (bind _returnvalue (`KismetSystemLibrary.K2_SetTimerDelegate` (`|CreateDelegate` :!event `CheckRagdollCanStop`) 1.0 true))
  (set `self.RagdollCheckHandle` _returnvalue)
  (`KismetSystemLibrary.K2_SetTimerDelegate` (`|CreateDelegate` :!event `CustomEvent`) (`self.RagdollMaxDuration`)))

(fn `UpdateActorLocationOnRagdoll`
  (`Actor.K2_SetActorLocationAndRotation` (`self.GetOwner` (`self.ref_mesh`)) (+ (.location (`self.RootTransform`)) (0.0 0.0 88.0)) (`KismetMathLibrary.MakeRotator` 0.0 0.0 (.yaw (.rotation (`self.RootTransform`)))) true false))