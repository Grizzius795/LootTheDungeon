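; BPC_Interactible is an actor component that makes its owner a hold-to-interact object with an optional highlight.
; Each BeginInteract call adds frame delta time to Progress until InteractDelay is reached, while ReleaseInteract resets it.
; On success, Progress resets and Interact fires the OnInteract dispatcher with the perpetrator.
; ToggleHighlight switches custom depth rendering and stencil value on all the owner's mesh components.
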(event `BeginInteract`
  (params (Perpetrator :type "Actor Object Reference"))
  (bind _output_get (set `self.Progress` (+ (`self.Progress`) (`GameplayStatics.GetWorldDeltaSeconds`))))
  (if (>= _output_get (`self.InteractDelay`))
    (`self.SucceedInteract` Perpetrator)))

(event `ReleaseInteract`
  (set `self.Progress` 0.0))

(event `SucceedInteract`
  (params (Perpetrator :type "Actor Object Reference"))
  (set `self.Progress` 0.0)
  (`self.Interact` Perpetrator))

(fn `Interact`
  (params (Perpetrator :type "Actor Object Reference"))
  (`self.OnInteract` Perpetrator))

(fn `ToggleHighlight`
  (params (Highlighted :type Boolean))
  (for _array_element (`Actor.K2_GetComponentsByClass` (`self.GetOwner`) "/Script/Engine.MeshComponent")
    (`PrimitiveComponent.SetRenderCustomDepth` _array_element (`local.Highlighted`))
    (`PrimitiveComponent.SetCustomDepthStencilValue` _array_element (`KismetMathLibrary.SelectInt` 1 0 (`local.Highlighted`)))))