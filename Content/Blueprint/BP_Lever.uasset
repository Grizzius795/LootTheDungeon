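; BP_Lever is an interactable lever that switches between on and off states.
; Its BPC_Interactible component's interact event calls Toggle, which plays the ActorSequence forward or in reverse, flips Activated and updates the action prompt text.
; A OneWay flag disables further interaction after a toggle, and an OnToggle dispatcher broadcasts the new state to listeners.
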(event `self.BPC_Interactible.OnInteract`
  (params (Perpetrator :type "Actor Object Reference"))
  (`self.Toggle`))

(event `Toggle`
  (bind _bpc_interactible (`self.BPC_Interactible`))
  (`|ExecutionSequence`
    (:`then_0`
      (if (`self.bActivated`)
        (`MovieSceneSequencePlayer.Play` (`ActorSequenceComponent.SequencePlayer` (`self.ActorSequence`)))
        (set `self.bActivated` false)
        (set `/Game/Blueprint/BPC_Interactible.ActionDescription` "Turn On" _bpc_interactible)
        (else
          (`MovieSceneSequencePlayer.PlayReverse` (`ActorSequenceComponent.SequencePlayer` (`self.ActorSequence`)))
          (set `self.bActivated` true)
          (set `/Game/Blueprint/BPC_Interactible.ActionDescription` "Turn Off" _bpc_interactible))))
    (:`then_1`
      (if (`self.bOneWay`)
        (set `/Game/Blueprint/BPC_Interactible.bInteractible` false (`self.BPC_Interactible`))))
    (:`then_2`
      (`self.OnToggle` (`self.bActivated`)))))

(fn `UserConstructionScript`)