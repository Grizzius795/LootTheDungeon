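; BP_WallBumper is a wall fist trap that knocks actors away.
; Overlapping Box plays the fist animation once, then after a short delay arms Bump for a brief window before a DoOnce resets.
; While armed, actors beginning overlap with Box1 receive a RagdollMessage with a strong impulse along the Arrow's forward vector.
; A Sequencer event spawns an attached Niagara dust cloud.
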(event `self.Box1.OnComponentBeginOverlap`
  (params (OverlappedComponent :type "PrimitiveComponent Object Reference") (OtherActor :type "Actor Object Reference") (OtherComp :type "PrimitiveComponent Object Reference") (OtherBodyIndex :type Integer) (bFromSweep :type Boolean) (SweepResult :type "HitResult Structure (by ref)"))
  (if (`self.bBump`)
    (message `/Game/Blueprint/Players/BPI_Attacks.Ragdoll` OtherActor (* (`SceneComponent.GetForwardVector` (`self.Arrow`)) 20000.0))))

(event `self.Box.OnComponentBeginOverlap`
  (params (OverlappedComponent :type "PrimitiveComponent Object Reference") (OtherActor :type "Actor Object Reference") (OtherComp :type "PrimitiveComponent Object Reference") (OtherBodyIndex :type Integer) (bFromSweep :type Boolean) (SweepResult :type "HitResult Structure (by ref)"))
  (`/Engine/EditorBlueprintResources/StandardMacros.DoOnce` false :!label _label
    (:`Completed`
      (`SkeletalMeshComponent.PlayAnimation` (`self.FistWall1`) "/Game/Blueprint/Trap/Bumper/FistWall1_Anim_Anim.FistWall1_Anim_Anim" false)
      (`KismetSystemLibrary.Delay` 0.5)
      (set `self.bBump` true)
      (`KismetSystemLibrary.Delay` 2.0)
      (set `self.bBump` false)
      (goto _label :!via `Reset`))))

(event `SequenceEvent`
  (`NiagaraFunctionLibrary.SpawnSystemAttached` "/Game/Blueprint/Trap/Bumper/NG_DustCloud.NG_DustCloud" null "None" (0.0 0.0 0.0) (struct) "KeepRelativeOffset" true))

(fn `UserConstructionScript`)