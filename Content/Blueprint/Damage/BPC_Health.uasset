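; Health component that tracks HP and damage per type, seeded from DT_DamageTypes, and raises take-damage, unconscious and death events.
; Bludgeoning and Slashing share one path: damage lowers HP, triggers unconsciousness at zero, and passes overflow on as Wound damage.
; Wounds leave HP untouched, eat into the other recorded damage in reverse key order, and cause death when their total reaches HPMax.
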(event `self.ReceiveBeginPlay`
  (set `self.HP` (`self.HP_max`))
  (`BlueprintMapLibrary.Map_Clear` (`self.Damages`))
  (bind _outrownames (`DataTableFunctionLibrary.GetDataTableRowNames` "/Game/Blueprint/Damage/DT_DamageTypes.DT_DamageTypes"))
  (for _array_element _outrownames
    (`BlueprintMapLibrary.Map_Add` (`self.Damages`) _array_element)))

(fn `Die`
  (`self.OnDeath`))

(fn `FallUnconscious`
  (`self.OnUnconscious`))

(fn `ModifyHP`
  (params (Amount :type Integer))
  (set `self.HP` (`KismetMathLibrary.Clamp` (+ (`self.HP`) Amount) 0 (`self.HP_max`))))

(fn `TakeBludgeoningDamage`
  (params (amount :type Integer) (Parameters :type "/Game/Blueprint/Damage/Struct_DamageParam Structure"))
  (returns (Out_Overdamage :type Integer))
  (locals (Overdamage :type Integer))
  (bind _returnvalue (- (`self.HP`) (`local.amount`)))
  (`|ExecutionSequence`
    (:`then_0`
      ; Calculate overdamage
      (if (< _returnvalue 0)
        (set `local.Overdamage` (`KismetMathLibrary.Abs_Int` _returnvalue))))
    (:`then_1`
      ; Loose HP
      (`BlueprintMapLibrary.Map_Add` (`self.Damages`) "Bludgeoning" (+ (`BlueprintMapLibrary.Map_Find` (`self.Damages`) "Bludgeoning") (`KismetMathLibrary.Clamp` (`local.Amount`) 0 (`self.HP`))))
      (`self.ModifyHP` (* (`local.amount`) -1)))
    (:`then_2`
      (if (<= (`self.HP`) 0)
        (`self.FallUnconscious`)))
    (:`then_3`
      (`self.OnTakeDamage`)
      (return (`local.Overdamage`)))))

(fn `TakeDamage`
  (params (DamageType :type Name) (Amount :type Integer) (parameters :type "/Game/Blueprint/Damage/Struct_DamageParam Structure"))
  (switch `name` DamageType
    (:`Default`
      (`KismetSystemLibrary.PrintString` "Invalid Damage Type" true true (struct :`R` 1.0 :`A` 1.0)))
    (:`Bludgeoning`
      (bind _out_overdamage (`self.TakeBludgeoningDamage` (`local.Amount`) (`local.parameters`) :!label _label))
      (`self.TakeWoundDamage` _out_overdamage (`local.parameters`)))
    (:`Slashing`
      (goto _label))
    (:`Wound`
      (`self.TakeWoundDamage` (`local.Amount`) (`local.parameters`)))))

(fn `TakeWoundDamage`
  (params (Amount :type Integer) (parameters :type "/Game/Blueprint/Damage/Struct_DamageParam Structure"))
  (locals (DamageList :type "Array of Name") (currentAmount :type Integer))
  (bind _damages (`self.Damages`))
  (set `local.currentAmount` Amount)
  (`|ExecutionSequence`
    (:`then_0`
      (bind _keys (`BlueprintMapLibrary.Map_Keys` (`self.Damages`)))
      (bind _output_get (set `local.DamageList` _keys))
      (`KismetArrayLibrary.Array_RemoveItem` _output_get "Wound")
      (`KismetArrayLibrary.Array_Reverse` _output_get)
      (for _array_element (`local.DamageList`)
        (if (> (`local.currentAmount`) 0)
          (bind _value (`BlueprintMapLibrary.Map_Find` (`self.Damages`) _array_element))
          (if (> _value 0)
            (`|ExecutionSequence`
              (:`then_0`
                (bind _returnvalue (- _value (`local.currentAmount`)))
                (if (< _returnvalue 0)
                  (set `local.currentAmount` (`KismetMathLibrary.Abs_Int` _returnvalue))))
              (:`then_1`
                (`BlueprintMapLibrary.Map_Add` (`self.Damages`) _array_element (`KismetMathLibrary.Clamp` _returnvalue 0 _value))))))))
    (:`then_1`
      (`BlueprintMapLibrary.Map_Add` _damages "Wound" (+ (`BlueprintMapLibrary.Map_Find` _damages "Wound") (`local.Amount`))))
    (:`then_2`
      (if (>= (`BlueprintMapLibrary.Map_Find` (`self.Damages`) "Wound") (`self.HP_max`))
        (`self.Die`)))
    (:`then_3`
      (`self.OnTakeDamage`))))