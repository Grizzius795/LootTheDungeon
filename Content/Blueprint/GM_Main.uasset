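; GM_Main is the main game mode, which spawns the mechanical door quest on begin play and stores it.
; It forwards player logins to BP_GameState after a short delay.
; It records each player's customization in a map and has the game state reapply all player appearances.
; A once-guarded event tells the game state to show the biome title card.
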(event `self.ReceiveBeginPlay`
  (bind _returnvalue (`|SpawnActorFromClass` "/Game/Blueprint/Quests/Quest_MecanicalDoor.Quest_MecanicalDoor_C" (`KismetMathLibrary.MakeTransform` (0.0 0.0 0.0)) "Undefined" "MultiplyWithRoot" null null))
  (set `self.Quest` _returnvalue))

(event `ShowBiomeTitleCard`
  (`/Engine/EditorBlueprintResources/StandardMacros.DoOnce` false
    (:`Completed`
      (bind _asbp_game_state (cast `/Game/Blueprint/BP_GameState` (`GameplayStatics.GetGameState`)))
      (`/Game/Blueprint/BP_GameState.ShowBiomeCard` _asbp_game_state))))

(event `self.K2_PostLogin`
  (params (NewPlayer :type "PlayerController Object Reference"))
  (`KismetSystemLibrary.Delay` 0.2)
  (bind _asbp_game_state (cast `/Game/Blueprint/BP_GameState` (`GameplayStatics.GetGameState`)))
  (`/Game/Blueprint/BP_GameState.PlayerLogin` _asbp_game_state NewPlayer))

(event `AddPlayerCustomization`
  (params (Player :type "/Game/Blueprint/Players/BP_AdventurerState Object Reference") (Customization :type "/Game/Blueprint/Mirror/Struct_CustomCharacter Structure"))
  (`BlueprintMapLibrary.Map_Add` (`self.PlayersCustomization`) Player Customization)
  (bind _asbp_game_state (cast `/Game/Blueprint/BP_GameState` (`GameplayStatics.GetGameState`)))
  (`/Game/Blueprint/BP_GameState.ApplyPlayerAppearances` _asbp_game_state))

(fn `UserConstructionScript`)