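; Dungeon generator Blueprint that generates on BeginPlay, building a rudimentary main path of a corridor start room plus one random room.
; CreateDungeon runs start, main path and finalize in sequence.
; The second room is placed at a random door position of the first with random cardinal rotation, always reporting success without requiring connection.
; ChooseDoor returns BP_Wall unless both rooms are valid, leaving connected openings without a door class.
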(event `self.ReceiveBeginPlay`
  (`self.Generate`))

(fn `AddNewRoom`
  (params (AdjacentRoom :type "Room Object Reference"))
  (returns (`New room` :type "Room Object Reference") (DoorToConnect :type Integer) (success :type Boolean))
  (locals (NewRoom :type "Room Object Reference") (tryCounter :type Integer) (L_DoorToConnect :type Integer :default 0))
  (bind _returnvalue (`self.CreateRoomInstance` (`KismetArrayLibrary.Array_Random` (`self.AvailableRooms`))))
  (set `local.NewRoom` _returnvalue)
  (`self.TryPlaceRoomAtTransform` (`local.NewRoom`) (make `RoomTransform` (`.Translation` (break `RoomTransform` (`.Transform` (break `DoorDef` (`KismetArrayLibrary.Array_Random` (`RoomData.Doors` (`ReadOnlyRoom.GetRoomData` (`local.AdjacentRoom`)))))))) (`KismetArrayLibrary.Array_Random` (`|MakeArray` "North" "East" "South" "West" :!type "EDoorDirection Enum"))))
  (if true
    _
    (else
      _))
  (return (`local.NewRoom`) (`local.L_DoorToConnect`) true))

(fn `ChooseDoor`
  (params (CurrentRoom :type "RoomData Object Reference") (CurrentRoomInstance :type "Room Object Reference") (NextRoom :type "RoomData Object Reference") (NextRoomInstance :type "Room Object Reference") (DoorType :type "DoorType Object Reference") (OtherDoorType :type "DoorType Object Reference"))
  (returns (Flipped :type Boolean) (ReturnValue :type "Actor Class Reference"))
  (if (and (`KismetSystemLibrary.IsValid` CurrentRoom) (`KismetSystemLibrary.IsValid` NextRoom))
    (return false null)
    (else
      (return false "/Game/Dungeon/Rooms/BP_Wall.BP_Wall_C"))))

(fn `CreateDungeon`
  (returns (ReturnValue :type Boolean))
  (`|ExecutionSequence`
    (:`then_0`
      (`self.StartNewDungeon`))
    (:`then_1`
      (`self.CreateMainPath`))
    (:`then_2`
      (`self.FinalizeDungeon`)
      (return true))))

(fn `CreateFirstRoom`
  (returns (Room :type "Room Object Reference"))
  (bind _returnvalue (`self.CreateRoomInstance` "/Game/Dungeon/Rooms/Test/RoomData_Corridor.RoomData_Corridor"))
  (`self.TryPlaceRoomAtTransform` _returnvalue)
  (`self.AddRoomToDungeon` :`Room` _returnvalue :`bFailIfNotConnected` false)
  (return _returnvalue))

(fn `CreateMainPath`
  (locals (NewRoom :type "Room Object Reference"))
  (bind _room (`self.CreateFirstRoom`))
  (bind _output_get (set `local.NewRoom` _room))
  (bind (_new_room _doortoconnect _success) (`self.AddNewRoom` _output_get))
  (if _success
    (`self.AddRoomToDungeon` :`Room` _new_room :`bFailIfNotConnected` false)))

(fn `UserConstructionScript`)