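; Procedural dungeon generator that grows a room graph from a first room until an end room is placed, then spawns players at BP_DungeonStart.
; It retries random content rooms for non-repetition, compatible doors and max count (always counting RoundStaircase), choosing the end room at corridor doors after a minimum room count.
; Validation requires a minimum start-to-end path length.
; DT_Doors supplies random doors by type, or walls for unconnected openings.
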(event `self.ReceiveBeginPlay`)

(event `self.OnPostGeneration`
  (bind _returnvalue (`GameplayStatics.GetActorOfClass` "/Game/Dungeon/Rooms/BP_DungeonStart.BP_DungeonStart_C"))
  (`/Engine/EditorBlueprintResources/StandardMacros.IsValid` _returnvalue
    (:`Is Valid`
      (`/Game/Dungeon/Rooms/BP_DungeonStart.SpawnPlayers` _returnvalue))))

(fn `ChooseDoor`
  (params (CurrentRoom :type "RoomData Object Reference") (CurrentRoomInstance :type "Room Object Reference") (NextRoom :type "RoomData Object Reference") (NextRoomInstance :type "Room Object Reference") (DoorType :type "DoorType Object Reference") (OtherDoorType :type "DoorType Object Reference"))
  (returns (Flipped :type Boolean) (ReturnValue :type "Actor Class Reference"))
  (locals (DoorData :type "/Game/Dungeon/Rooms/Struct_Door Structure"))
  (set `local.DoorData` (`self.GetDoorTypeData` (`local.DoorType`)))
  (if (and (`KismetSystemLibrary.IsValid` CurrentRoom) (`KismetSystemLibrary.IsValid` NextRoom))
    (return false (`KismetArrayLibrary.Array_Random` (`.Doors_8_487989674DE0DBB2A211B8837BD728C7` (break `/Game/Dungeon/Rooms/Struct_Door` (`local.DoorData`)))))
    (else
      (return false (`KismetArrayLibrary.Array_Random` (`.Walls_9_B5CB6FB849BDE56D6D9250A2AC60A0A3` (break `/Game/Dungeon/Rooms/Struct_Door` (`local.DoorData`))))))))

(fn `ChooseFirstRoomData`
  (returns (Transform :type "RoomTransform Structure") (ReturnValue :type "RoomData Object Reference"))
  (return (struct) (`self.FirstRoom`)))

(fn `ChooseNextRoomData`
  (params (CurrentRoom :type "RoomData Object Reference") (CurrentRoomInstance :type "ReadOnlyRoom Interface (by ref)") (DoorData :type "DoorDef Structure (by ref)"))
  (returns (DoorIndex :type Integer) (ReturnValue :type "RoomData Object Reference"))
  (locals (NewRoom :type "RoomData Object Reference"))
  (if (>= (`DungeonGraph.Count` (`self.Graph`)) (`self.MinNbRooms`))
    (if (== (`.Type` (break `DoorDef` (`local.DoorData`))) "/Game/Dungeon/Rooms/LushLabyrinth/Doors/Door_Corridor.Door_Corridor")
      (return 0 (`self.EndRoom`))
      (else
        _)))
  (bind _returnvalue (`self.GetRandomRoomData` (`self.ContentRooms`) :!label _label))
  (set `local.NewRoom` _returnvalue)
  (if (and (!= (`local.NewRoom`) (`local.CurrentRoom`)) (`self.RoomMeetsMaxCount` (`local.NewRoom`)) (> (`KismetArrayLibrary.Array_Length` (`RoomData.GetCompatibleDoors` (`local.NewRoom`) (`local.DoorData`))) 0))
    (return -1 (`local.NewRoom`))
    (else
      (goto _label))))

(fn `ContinueToAddRoom`
  (returns (ReturnValue :type Boolean))
  (return (not (`DungeonGraph.HasAlreadyRoomData` (`self.Graph`) (`self.EndRoom`)))))

(fn `GetDoorTypeData`
  (params (DoorType :type "Object Object Reference"))
  (returns (Data :type "/Game/Dungeon/Rooms/Struct_Door Structure"))
  (bind _outrownames (`DataTableFunctionLibrary.GetDataTableRowNames` "/Game/Dungeon/Rooms/DT_Doors.DT_Doors"))
  (for _array_element _outrownames
    (bind _returnvalue (`|GetDataTableRow` "/Game/Dungeon/Rooms/DT_Doors.DT_Doors" _array_element)
      (:`then`
        (if (== (`.DoorType_2_E555F705418FC125B1220792C40D32CB` (break `/Game/Dungeon/Rooms/Struct_Door` _returnvalue)) DoorType)
          (return _returnvalue))))))

(fn `IsValidDungeon`
  (returns (ReturnValue :type Boolean))
  (locals (FirstRoom :type "Room Object Reference") (FinalRoom :type "Room Object Reference"))
  (`|ExecutionSequence`
    (:`then_0`
      (bind _rooms (`DungeonGraph.GetAllRoomsFromData` (`self.Graph`) (`self.FirstRoom`)))
      (set `local.FirstRoom` (`|GetArrayItem` _rooms))
      (bind _rooms_2 (`DungeonGraph.GetAllRoomsFromData` (`self.Graph`) (`self.EndRoom`)))
      (set `local.FinalRoom` (`|GetArrayItem` _rooms_2)))
    (:`then_1`
      (bind (_resultpath _returnvalue) (`DungeonGraph.GetPathBetween` (`self.Graph`) (`local.FirstRoom`) (`local.FinalRoom`) false))
      (if _returnvalue
        (return (>= (`KismetArrayLibrary.Array_Length` _resultpath) (`self.MinLength`)))
        (else
          (return false))))))

(fn `RoomMeetsMaxCount`
  (params (RoomData :type "RoomData Object Reference"))
  (returns (Out :type Boolean))
  (locals (L_RoomData :type "/Game/Dungeon/Rooms/DungeonRoomData Object Reference"))
  (bind _asdungeon_room_data (cast `/Game/Dungeon/Rooms/DungeonRoomData` RoomData))
  (set `local.L_RoomData` _asdungeon_room_data)
  (if (> (`/Game/Dungeon/Rooms/DungeonRoomData.MaxCount` _asdungeon_room_data) 0)
    (bind _rooms (`DungeonGraph.GetAllRoomsFromData` (`self.Graph`) "/Game/Dungeon/Rooms/Test/RoomData_RoundStaircase.RoomData_RoundStaircase"))
    (return (< (`KismetArrayLibrary.Array_Length` _rooms) (`/Game/Dungeon/Rooms/DungeonRoomData.MaxCount` (`local.L_RoomData`))))
    (else
      (return true))))

(fn `UserConstructionScript`)